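; Hunger and thirst component for player characters, draining food and drink on a looping server timer.
; Drain scales with Metabolism, server settings and active, idle (full stamina) or offline state, and drops sharply inside shelter.
; Server events handle eating and drinking; full meters pause drain with timed Sated/Hydrated buffs unless food-poisoned, while empty meters add Hungry/Thirsty.
; RepNotifies signal value changes; literal amounts and debug tick toggles are admin-only.
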(event EventDataLoaded
  (bind _returnvalue (Components|GetOwner))
  (bind (_asbase_bpchar _bsuccess) (Utilities|Casting|CastToBaseBPChar _returnvalue))
  (Utilities|FlowControl|Sequence
    (:then_0
      (if _bsuccess
        (bind _output_get (Variables|Default|SetBasePlayerChar _asbase_bpchar))
        (Utilities|FlowControl|Sequence
          (:then_0
            (if (> (Utilities|Array|Length (Actor|GetComponentsByClass _output_get "/Game/Systems/Buffs/00_BP_AC_BuffSystem.00_BP_AC_BuffSystem_C")) 0)
              (Variables|Components|SetBuffSystem (Utilities|Array|Get(acopy) (Actor|GetComponentsByClass _output_get "/Game/Systems/Buffs/00_BP_AC_BuffSystem.00_BP_AC_BuffSystem_C")))
              (else
                (Class|LoggerLibrary|DWLogString "BP_HungerSystem unable to get Buff System component." "Combat" "INFOL_DATAWARNING"))))
          (:then_1
            (if (> (Utilities|Array|Length (Actor|GetComponentsByClass _output_get "/Game/Systems/Progression/BP_ProgressionSystem.BP_ProgressionSystem_C")) 0)
              (Variables|Components|SetProgressionSystem (Utilities|Array|Get(acopy) (Actor|GetComponentsByClass _output_get "/Game/Systems/Progression/BP_ProgressionSystem.BP_ProgressionSystem_C")))
              (else
                (Class|LoggerLibrary|DWLogString "BP_HungerSystem unable to get Progression System component." "Combat" "INFOL_DATAWARNING")))))
        (else
          (Development|PrintString (Utilities|String|ToString(Text) (Utilities|Text|FormatText "{name} FAILED TO CAST IN BP_HUNGERSYSTEM, THIS SHOULD NEVER HAPPEN" (Utilities|Text|ToText(String) (Utilities|GetObjectName (Components|GetOwner)))))))))
    (:then_1
      (if (Networking|IsServer)
        (Utilities|Time|SetTimerbyFunctionName self "HungerSystemTick" (Variables|System|GetSystemTickRate) true)))))

(event Custom|ServerGiveFood
  (params (FromGameItem :type Game%20Item%20Object%20Reference) (LiteralFoodAmt :type Float%20%28single-precision%29))
  ;[1 1 1] Eating and drinking.  Also accepts literal values from the Admin Panel
  (Utilities|IsValid FromGameItem
    (:Is%20Valid
      (Food|HandleFoodConsume (Math|Conversions|ToFloat(Integer) (Class|GameItem|GetIntStat FromGameItem "FoodAmount"))))
    (:Is%20Not%20Valid
      (Utilities|IsAdmin
        (:True
          (Food|HandleFoodConsume LiteralFoodAmt))))))

(event Custom|ServerGiveDrink
  (params (FromGameItem :type Game%20Item%20Object%20Reference) (LiteralDrinkAmount :type Float%20%28single-precision%29))
  ;[1 1 1] Eating and drinking.  Also accepts literal values from the Admin Panel
  (Utilities|IsValid FromGameItem
    (:Is%20Valid
      (Drink|HandleDrinkConsume (* (Variables|/Game/Systems/BP_ServerSettings.BP_ServerSettings_C|GetPlayerWaterMultiplier (|GetServerSettings)) (Math|Conversions|ToFloat(Integer) (Class|GameItem|GetIntStat FromGameItem "DrinkAmount")))))
    (:Is%20Not%20Valid
      (Utilities|IsAdmin
        (:True
          (Drink|HandleDrinkConsume LiteralDrinkAmount))))))

(event Custom|MulticastStartDrinkFromWaterSource
  (params (Player :type Base%20BP%20Char%20Object%20Reference))
  ;[1 1 1] Move this server and client function to base player char where all the others are implemented
  (bind _isremote (Default|IsRemoteActor Player))
  (if _isremote
    (CallFunction|ClientDrinkfromWaterSource Player)))

(event Custom|ServerDebugDrinkTickDisable
  ;[1 1 1] Debug Server Commands
  (Utilities|IsAdmin
    (:True
      (Variables|Default|SetDebugDrinkTickEnabled false))))

(event Custom|ServerDebugFoodTickDisable
  ;[1 1 1] Debug Server Commands
  (Utilities|IsAdmin
    (:True
      (Variables|Default|SetDebugFoodTickEnabled false))))

(event Custom|ServerDebugFoodTickEnabled
  ;[1 1 1] Debug Server Commands
  (Utilities|IsAdmin
    (:True
      (Variables|Default|SetDebugFoodTickEnabled true))))

(event Custom|ServerDebugDrinkTickEnabled
  ;[1 1 1] Debug Server Commands
  (Utilities|IsAdmin
    (:True
      (Variables|Default|SetDebugDrinkTickEnabled true))))

(event Custom|ServerStartDrinkFromWaterSource
  ;[1 1 1] Move this server and client function to base player char where all the others are implemented
  (Drink|HandleDrinkConsume 3e+01)
  (CallFunction|MulticastStartDrinkfromWaterSource (Variables|Default|GetBasePlayerChar)))

(fn HandleFoodTick
  (if (Variables|Default|GetDebugFoodTickEnabled)
    (if (not (Variables|Food|GetisSated))
      (bind _foodconsumemultiplier (CallFunction|SetConsumeRates))
      (bind _out (CallFunction|ModifyifInsideShelter _foodconsumemultiplier))
      (bind _value (CallFunction|GetFoodCurrent))
      (Food|SetFoodCurrent (Math|Float|Clamp(Float) (- _value (* _out (Food|GetFoodConsume))) 0.0 (Food|GetFoodMax)))
      (Food|HandleNoFood))))

(fn HandleDrinkTick
  (if (Variables|Default|GetDebugDrinkTickEnabled)
    (if (not (Variables|Drink|GetisHydrated))
      (bind _drinkconsumemultiplier (CallFunction|SetConsumeRates))
      (bind _out (CallFunction|ModifyifInsideShelter _drinkconsumemultiplier))
      (bind _value (CallFunction|GetDrinkCurrent))
      (Drink|SetDrinkCurrent (Math|Float|Clamp(Float) (- _value (* _out (Drink|GetDrinkConsume))) 0.0 (Drink|GetDrinkMax)))
      (Drink|HandleNoDrink))))

(fn HandleFoodConsume
  (params (food :type Float%20%28single-precision%29))
  (Food|IncreaseFood food)
  (Food|HandleSated))

(fn HandleDrinkConsume
  (params (Drink :type Float%20%28single-precision%29))
  (Drink|IncreaseDrink Drink)
  (Drink|HandleHydrated))

(fn UnpauseConsumeFoodTimer
  (Variables|Food|SetisSated false)
  (Default|RemoveBuff (Variables|Components|GetBuffSystem) (Variables|Default|GetBuffSated) (Variables|Default|GetBasePlayerChar)))

(fn UnpauseConsumeDrinkTimer
  (Variables|Drink|SetisHydrated false)
  (Default|RemoveBuff (Variables|Components|GetBuffSystem) (Variables|Default|GetBuffHydrated) (Variables|Default|GetBasePlayerChar)))

(fn GetDrinkMax
  (return (Variables|Drink|GetDrinkMax)))

(fn GetDrinkConsume
  (bind _progressionsystem (Variables|Components|GetProgressionSystem))
  (return (- (Variables|Drink|ConsumeValues|GetDrinkConsumeMax) (* (Variables|/Game/Systems/Progression/BP_ProgressionSystem.BP_ProgressionSystem_C|GetAttributeMetabolism _progressionsystem) (/ (- (Variables|Drink|ConsumeValues|GetDrinkConsumeMax) (Variables|Drink|ConsumeValues|GetDrinkConsumeMin)) (Math|Conversions|ToFloat(Integer) (Variables|/Game/Systems/Progression/BP_ProgressionSystem.BP_ProgressionSystem_C|GetMaxAttributePointsSpent _progressionsystem)))))))

(fn GetFoodMax
  (return (Variables|Food|GetFoodMax)))

(fn GetFoodConsume
  (bind _progressionsystem (Variables|Components|GetProgressionSystem))
  (return (- (Variables|Food|ConsumeValues|GetFoodConsumeMax) (* (Variables|/Game/Systems/Progression/BP_ProgressionSystem.BP_ProgressionSystem_C|GetAttributeMetabolism _progressionsystem) (/ (- (Variables|Food|ConsumeValues|GetFoodConsumeMax) (Variables|Food|ConsumeValues|GetFoodConsumeMin)) (Math|Conversions|ToFloat(Integer) (Variables|/Game/Systems/Progression/BP_ProgressionSystem.BP_ProgressionSystem_C|GetMaxAttributePointsSpent _progressionsystem)))))))

(fn SetDrinkCurrent
  (params (value :type Float%20%28single-precision%29))
  (Variables|Drink|SetDrinkCurrent value)
  (return))

(fn SetFoodCurrent
  (params (value :type Float%20%28single-precision%29))
  (Variables|Food|SetFoodCurrent value)
  (return))

(fn HandleSated
  (if (> (Utilities|Array|Length (Actor|GetComponentsByClass (Components|GetOwner) (Variables|Default|GetBuffFoodPoisoning))) 0)
    (Food|UnpauseConsumeFoodTimer)
    (else
      (bind _value (CallFunction|GetFoodCurrent))
      (if (Math|Float|NearlyEqual(Float) _value (Food|GetFoodMax) 1e-06)
        (Utilities|FlowControl|Sequence
          (:then_0
            (Variables|Food|SetisSated true)
            (bind _returnvalue (Utilities|Time|SetTimerbyFunctionName self "UnpauseConsumeFoodTimer" (Food|GetSatedDuration)))
            (Variables|Food|SetSatedTimer _returnvalue))
          (:then_1
            (Default|AddBuff (Variables|Components|GetBuffSystem) (Variables|Default|GetBuffSated) (Variables|Default|GetBasePlayerChar))))))))

(fn HandleHydrated
  (if (> (Utilities|Array|Length (Actor|GetComponentsByClass (Components|GetOwner) (Variables|Default|GetBuffFoodPoisoning))) 0)
    (Drink|UnpauseConsumeDrinkTimer)
    (else
      (bind _value (CallFunction|GetDrinkCurrent))
      (if (Math|Float|NearlyEqual(Float) _value (Drink|GetDrinkMax) 1e-06)
        (Utilities|FlowControl|Sequence
          (:then_0
            (Variables|Drink|SetisHydrated true)
            (bind _returnvalue (Utilities|Time|SetTimerbyFunctionName self "UnpauseConsumeDrinkTimer" (Drink|GetHydratedDuration)))
            (Variables|Drink|SetHydratedTimer _returnvalue))
          (:then_1
            (Default|AddBuff (Variables|Components|GetBuffSystem) (Variables|Default|GetBuffHydrated) (Variables|Default|GetBasePlayerChar))))))))

(fn HandleNoFood
  (bind _value (CallFunction|GetFoodCurrent))
  (if (Math|Float|NearlyEqual(Float) _value 0.0 1e-06)
    (Food|SetFoodDepleted true)))

(fn HandleNoDrink
  (bind _value (CallFunction|GetDrinkCurrent))
  (if (Math|Float|NearlyEqual(Float) _value 0.0 1e-06)
    (Drink|SetDrinkDepleted true)))

(fn IncreaseFood
  (params (gain :type Float%20%28single-precision%29))
  (bind _value (CallFunction|GetFoodCurrent))
  (Food|SetFoodCurrent (Math|Float|Clamp(Float) (+ _value gain) 0.0 (Food|GetFoodMax)))
  (bind _value_2 (CallFunction|GetFoodCurrent))
  (if (!= _value_2 0.0)
    (Food|SetFoodDepleted false)))

(fn IncreaseDrink
  (params (gain :type Float%20%28single-precision%29))
  (bind _value (CallFunction|GetDrinkCurrent))
  (Drink|SetDrinkCurrent (Math|Float|Clamp(Float) (+ _value gain) 0.0 (Drink|GetDrinkMax)))
  (bind _value_2 (CallFunction|GetDrinkCurrent))
  (if (!= _value_2 0.0)
    (Drink|SetDrinkDepleted false)))

(fn IsDying
  (return (or (Food|GetFoodDepleted) (Drink|GetDrinkDepleted))))

(fn SetFoodDepleted
  (params (value :type Boolean))
  (bind _output_get (Variables|Food|SetisFoodDepleted value))
  (if _output_get
    (Default|AddBuff (Variables|Components|GetBuffSystem) (Variables|Default|GetBuffHungry) (Variables|Default|GetBasePlayerChar))
    (else
      (Default|RemoveBuff (Variables|Components|GetBuffSystem) (Variables|Default|GetBuffHungry) (Variables|Default|GetBasePlayerChar)))))

(fn SetDrinkDepleted
  (params (value :type Boolean))
  (bind _output_get (Variables|Drink|SetisDrinkDepleted value))
  (if _output_get
    (Default|AddBuff (Variables|Components|GetBuffSystem) (Variables|Default|GetBuffThirsty) (Variables|Default|GetBasePlayerChar))
    (else
      (Default|RemoveBuff (Variables|Components|GetBuffSystem) (Variables|Default|GetBuffThirsty) (Variables|Default|GetBasePlayerChar)))))

(fn GetFoodDepleted
  (return (Variables|Food|GetisFoodDepleted)))

(fn GetDrinkDepleted
  (return (Variables|Drink|GetisDrinkDepleted)))

(fn GetSatedDuration
  (return (* (Variables|Food|GetSatedDuration) (- 1.0 (Variables|/Game/Systems/Progression/BP_ProgressionSystem.BP_ProgressionSystem_C|GetBonusHungerBuffDurationModifier (Variables|Components|GetProgressionSystem))))))

(fn GetHydratedDuration
  (return (* (Variables|Drink|GetHydratedDuration) (- 1.0 (Variables|/Game/Systems/Progression/BP_ProgressionSystem.BP_ProgressionSystem_C|GetBonusHungerBuffDurationModifier (Variables|Components|GetProgressionSystem))))))

(fn ClientDrinkfromWaterSource
  (params (Player :type Base%20BP%20Char%20Object%20Reference))
  (Default|EnterSubstate Player "NewEnumerator4"))

(fn SetConsumeRates
  (bind _returnvalue (|GetServerSettings))
  (bind _returnvalue_2 (|GetServerSettings))
  (bind _returnvalue_3 (|GetServerSettings))
  (bind _returnvalue_4 (Components|GetOwner))
  (bind _returnvalue_5 (Actor|GetComponentsByClass _returnvalue_4 "/Script/ConanSandbox.StatHolder"))
  (bind _item (Utilities|Array|Get(acopy) _returnvalue_5))
  (if (> (Utilities|Array|Length _returnvalue_5) 0)
    (bind _aspawn (Utilities|Casting|CastToPawn _returnvalue_4)
      (:then
        (if (Pawn|IsPlayerControlled _aspawn)
          (if (< (Class|StatHolder|GetIntStat _item "StaminaCurrent" "Full") (Class|StatHolder|GetIntStat _item "StaminaMax" "Full"))
            ;[1 0.737 0.3437] Set Active Consume Rate
            (Utilities|IsValid _returnvalue_3
              (:Is%20Valid
                (return (* (* (Drink|GetDrinkConsumeRate) (Variables|Drink|ConsumeValues|GetDrinkConsumeActiveMultiplier)) (Variables|/Game/Systems/BP_ServerSettings.BP_ServerSettings_C|GetPlayerActiveThirstMultiplier _returnvalue_3)) (* (* (Food|GetFoodConsumeRate) (Variables|Food|ConsumeValues|GetFoodConsumeActiveMultiplier)) (Variables|/Game/Systems/BP_ServerSettings.BP_ServerSettings_C|GetPlayerActiveHungerMultiplier _returnvalue_3))))
              (:Is%20Not%20Valid
                _))
            (else
              ;[1 1 1] Set Idle Consume Rate
              (Utilities|IsValid _returnvalue_2
                (:Is%20Valid
                  (return (* (* (Drink|GetDrinkConsumeRate) (Variables|Drink|ConsumeValues|GetDrinkConsumeIdleMultiplier)) (Variables|/Game/Systems/BP_ServerSettings.BP_ServerSettings_C|GetPlayerIdleThirstMultiplier _returnvalue_2)) (* (* (Food|GetFoodConsumeRate) (Variables|Food|ConsumeValues|GetFoodConsumeIdleMultiplier)) (Variables|/Game/Systems/BP_ServerSettings.BP_ServerSettings_C|GetPlayerIdleHungerMultiplier _returnvalue_2))))
                (:Is%20Not%20Valid
                  _))))
          (else
            ;[1 0.2668 0.217] Set Offline Consume Rate
            (Utilities|IsValid _returnvalue
              (:Is%20Valid
                (return (* (* (Drink|GetDrinkConsumeRate) (Variables|Drink|ConsumeValues|GetDrinkConsumeOfflineMultiplier)) (Variables|/Game/Systems/BP_ServerSettings.BP_ServerSettings_C|GetPlayerOfflineThirstMultiplier _returnvalue)) (* (* (Food|GetFoodConsumeRate) (Variables|Food|ConsumeValues|GetFoodConsumeOfflineMultiplier)) (Variables|/Game/Systems/BP_ServerSettings.BP_ServerSettings_C|GetPlayerOfflineHungerMultiplier _returnvalue))))
              (:Is%20Not%20Valid
                _))))
        (Class|LoggerLibrary|DWLogString (Utilities|String|Append "BP_HungerSystem for actor " (Utilities|GetDisplayName (Components|GetOwner)) "cannot find valid ServerSettings in Set Consume Rates") "Combat" "INFOL_DATAERROR")
        (return 1.0 1.0))
      (:CastFailed
        (return 1.0 1.0)))
    (else
      (Class|LoggerLibrary|DWLogString (Utilities|String|Append "BP_HungerSystem for actor " (Utilities|GetDisplayName (Components|GetOwner)) " cannot find actorcomponent StatHolder in \"Set Consume Rates\" function.") "Combat" "INFOL_DATAERROR")
      (return 1.0 1.0))))

(fn GetDrinkConsumeRate
  (return (/ (Variables|Drink|GetDrinkMax) (* (Variables|Drink|ConsumeValues|GetDrinkConsumeBase) 6e+01))))

(fn GetFoodConsumeRate
  (return (/ (Variables|Food|GetFoodMax) (* (Variables|Food|ConsumeValues|GetFoodConsumeBase) 6e+01))))

(fn OnRepFoodCurrent
  (Default|CallSignalHungerChanged (Variables|Food|GetFoodCurrent) (Variables|Food|GetFoodMax)))

(fn OnRepDrinkCurrent
  (Default|CallSignalThirstChanged (Variables|Drink|GetDrinkCurrent) (Variables|Drink|GetDrinkMax)))

(fn HungerSystemTick
  (Drink|HandleDrinkTick)
  (Food|HandleFoodTick))

(fn ModifyifInsideShelter
  (params (In :type Float%20%28single-precision%29))
  (bind _returnvalue (Components|GetOwner))
  (bind _returnvalue_2 (Actor|GetComponentsByClass _returnvalue "/Game/Systems/Building/InsideChecker.InsideChecker_C"))
  ;[1 1 1] Severly reduced food/drink consume rate if inside shelter
  (if (> (Utilities|Array|Length _returnvalue_2) 0)
    (if (>= (Variables|/Game/Systems/Building/InsideChecker.InsideChecker_C|GetInsidePercentage (Utilities|Array|Get(acopy) _returnvalue_2)) 1.0)
      (return (* In 0.1))
      (else
        _)))
  (return In))

(fn GetDrinkCurrent
  (return (Variables|Drink|GetDrinkCurrent)))

(fn GetFoodCurrent
  (return (Variables|Food|GetFoodCurrent)))