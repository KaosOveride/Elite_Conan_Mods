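; Camp component that manages a group of camp actors, their respawning, and exposes their spawn points and waypoints.
; On server BeginPlay it registers with the GameMode's CampSystem component, retrying if absent.
; Destroyed actors enter a delayed respawn queue gated by nearby players and building land claims, which deactivate the camp and start periodic reactivation checks.
; Camps with essential actors stop providing navigation when none remain, unless forced active; debug strings report state.
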(event Custom|Camper_Destroyed
  (params (DestroyedActor :type Actor%20Object%20Reference))
  (bind _returnvalue (Utilities|GetClass DestroyedActor))
  (bind _returnvalue_2 (Transformation|GetActorTransform DestroyedActor))
  (bind _returnvalue_3 (Utilities|Time|GetRealTimeSeconds))
  (bind _campsystem (Variables|Camps|GetCampSystem))
  (bind _campessentials (Variables|Camps|GetCampEssentials))
  (bind _respawningactors (Variables|Camps|GetRespawningActors))
  (bind _respawningactors_2 (Variables|Camps|GetRespawningActors))
  (bind _item (Utilities|Array|Get(acopy) _respawningactors))
  (bind _camprespawntime (Variables|/Game/Systems/Camps/BP_CampSystemComponent.BP_CampSystemComponent_C|GetCampRespawnTime _campsystem))
  (bind (_class _transform) (Utilities|Struct|BreakST_CampActor _item))
  (bind (_class_2 _transform_2) (Utilities|Struct|BreakST_CampActor _item))
  (bind _returnvalue_4 (+ _returnvalue_3 _camprespawntime))
  (bind _location (Math|Transform|BreakTransform _transform_2))
  (bind _st_campactor (Utilities|Struct|MakeST_CampActor _returnvalue _returnvalue_2 _returnvalue_4))
  ;[1 1 1] CampActor destroyed. If the camp is active, start the respawn timer
  (Utilities|Array|RemoveItem (Variables|Camps|GetCampActors) DestroyedActor)
  (Utilities|Array|RemoveItem _campessentials DestroyedActor)
  (if (and (Variables|Camps|GetHasCampEssentials) (<= (Utilities|Array|Length _campessentials) 0))
    (CallFunction|SetCampActiveState (Variables|Camps|GetIsCampActive) "NewEnumerator3"))
  (if (Variables|Camps|GetIsCampActive)
    (Utilities|Array|Add (Variables|Camps|GetRespawningActors) _st_campactor)
    (if (< (Variables|Camps|GetCurrentRespawnTargetTime) (Utilities|Time|GetRealTimeSeconds))
      (Variables|Camps|SetCurrentRespawnTargetTime (+ (Utilities|Time|GetRealTimeSeconds) (Variables|/Game/Systems/Camps/BP_CampSystemComponent.BP_CampSystemComponent_C|GetCampRespawnTime (Variables|Camps|GetCampSystem)))))
    (bind _returnvalue_5 (Class|LandClaimSystem|CanClaimSphere "Building" (Utilities|Struct|MakeClaimOwnershipParams (Class|UniqueID|MakeNullUID)) (.Location (Math|Transform|BreakTransform (.Transform (Utilities|Struct|BreakST_CampActor (Utilities|Array|Get(acopy) (Variables|Camps|GetRespawningActors)))))) (Variables|Default|GetPlayerBuilt_Claim_Radius)))
    (if _returnvalue_5
      (bind _returnvalue_6 (Utilities|Time|SetTimerbyEvent (delegate Custom|CheckForLandclaim) 1.2e+02 true))
      (Variables|Default|SetLandClaimChecker _returnvalue_6)
      (Utilities|FlowControl|Delay (- (Variables|Camps|GetCurrentRespawnTargetTime) (Utilities|Time|GetRealTimeSeconds)) :!label _label)
      (if (Variables|Camps|GetIsCampActive)
        (bind _returnvalue_7 (Class|LandClaimSystem|CanClaimSphere "Building" (Utilities|Struct|MakeClaimOwnershipParams (Class|UniqueID|MakeNullUID)) _location (Variables|Default|GetPlayerBuilt_Claim_Radius)))
        (if _returnvalue_7
          (bind _returnvalue_8 (Class|PlayerPawnRegistry|HasPawnWithinDistance (Variables|Camps|GetPlayerPawnRegistry) _location (Variables|/Game/Systems/Camps/BP_CampSystemComponent.BP_CampSystemComponent_C|GetCampRespawnExclusionRadius (Variables|Camps|GetCampSystem))))
          (if _returnvalue_8
            ;[1 1 1] Players too close, add to respawn queue and try again
            (Utilities|Array|Add (Variables|Camps|GetRespawningActors) (Utilities|Struct|MakeST_CampActor _class _transform (+ (Utilities|Time|GetRealTimeSeconds) (Variables|/Game/Systems/Camps/BP_CampSystemComponent.BP_CampSystemComponent_C|GetCampRespawnTime (Variables|Camps|GetCampSystem)))))
            (else
              (bind _spawnedactor (CallFunction|SpawnCampActor _class_2 _transform_2))
              (Game|BindEventtoOnDestroyed _spawnedactor (delegate Custom|Camper_Destroyed))))
          (else
            ;[1 1 1] Deactivate camp and start landclaim retrying (will do some rare checks)
            (CallFunction|SetCampActiveState false "NewEnumerator5")
            (CallFunction|DeactivatedDuetoLandClaim)
            (Utilities|Array|Add (Variables|Camps|GetDestroyedActors) _item :!label _label_2)))
        (else
          (goto _label_2)))
      ;[1 1 1] Remove the last respawn attempt, and go to the next one in the queue.
      (Utilities|Array|RemoveIndex (Variables|Camps|GetRespawningActors))
      (if (> (Utilities|Array|Length _respawningactors_2) 0)
        (Variables|Camps|SetCurrentRespawnTargetTime (.RespawnTime (Utilities|Struct|BreakST_CampActor (Utilities|Array|Get(acopy) _respawningactors_2))))
        (goto _label))
      (else
        (CallFunction|DeactivateCamp)))
    (else
      (Utilities|Array|Add (Variables|Camps|GetDestroyedActors) _st_campactor))))

(event Custom|CheckForLandclaim
  ;[1 1 1] If a camp asset is respawning, start a seperate timer to check landclaim for respawning campactors so npcs can stop respawning if a building is built nearby. (workaround)
  (if (> (Utilities|Array|Length (Variables|Camps|GetRespawningActors)) 0)
    (bind _array_element (Utilities|Array|ForEachLoopwithBreak (Variables|Camps|GetRespawningActors) :!label _label)
      (:LoopBody
        (bind _returnvalue (Class|LandClaimSystem|CanClaimSphere "Building" (Utilities|Struct|MakeClaimOwnershipParams (Class|UniqueID|MakeNullUID)) (.Location (Math|Transform|BreakTransform (.Transform (Utilities|Struct|BreakST_CampActor _array_element)))) (Variables|Default|GetPlayerBuilt_Claim_Radius)))
        (if (not _returnvalue)
          (CallFunction|DeactivateCamp)
          (goto _label Break))))
    (else
      (Utilities|Time|ClearandInvalidateTimerbyHandle (Variables|Default|GetLandClaimChecker)))))

(event Custom|DeactivateCamp
  (bind _respawningactors (Variables|Camps|GetRespawningActors))
  (bind _respawningactors_2 (Variables|Camps|GetRespawningActors))
  (bind _item (Utilities|Array|Get(acopy) _respawningactors))
  (bind (_class _transform) (Utilities|Struct|BreakST_CampActor _item))
  (bind (_class_2 _transform_2) (Utilities|Struct|BreakST_CampActor _item))
  (bind _location (Math|Transform|BreakTransform _transform_2))
  ;[1 1 1] Deactivate camp and start landclaim retrying (will do some rare checks)
  (CallFunction|SetCampActiveState false "NewEnumerator5" :!label _label)
  (CallFunction|DeactivatedDuetoLandClaim)
  (Utilities|Array|Add (Variables|Camps|GetDestroyedActors) _item :!label _label_2)
  ;[1 1 1] Remove the last respawn attempt, and go to the next one in the queue.
  (Utilities|Array|RemoveIndex (Variables|Camps|GetRespawningActors) :!label _label_3)
  (if (> (Utilities|Array|Length _respawningactors_2) 0)
    (Variables|Camps|SetCurrentRespawnTargetTime (.RespawnTime (Utilities|Struct|BreakST_CampActor (Utilities|Array|Get(acopy) _respawningactors_2))))
    (Utilities|FlowControl|Delay (- (Variables|Camps|GetCurrentRespawnTargetTime) (Utilities|Time|GetRealTimeSeconds)))
    (if (Variables|Camps|GetIsCampActive)
      (bind _returnvalue (Class|LandClaimSystem|CanClaimSphere "Building" (Utilities|Struct|MakeClaimOwnershipParams (Class|UniqueID|MakeNullUID)) _location (Variables|Default|GetPlayerBuilt_Claim_Radius)))
      (if _returnvalue
        (bind _returnvalue_2 (Class|PlayerPawnRegistry|HasPawnWithinDistance (Variables|Camps|GetPlayerPawnRegistry) _location (Variables|/Game/Systems/Camps/BP_CampSystemComponent.BP_CampSystemComponent_C|GetCampRespawnExclusionRadius (Variables|Camps|GetCampSystem))))
        (if _returnvalue_2
          ;[1 1 1] Players too close, add to respawn queue and try again
          (Utilities|Array|Add (Variables|Camps|GetRespawningActors) (Utilities|Struct|MakeST_CampActor _class _transform (+ (Utilities|Time|GetRealTimeSeconds) (Variables|/Game/Systems/Camps/BP_CampSystemComponent.BP_CampSystemComponent_C|GetCampRespawnTime (Variables|Camps|GetCampSystem)))))
          (goto _label_3)
          (else
            (bind _spawnedactor (CallFunction|SpawnCampActor _class_2 _transform_2))
            (Game|BindEventtoOnDestroyed _spawnedactor (delegate Custom|Camper_Destroyed))
            (goto _label_3)))
        (else
          (goto _label)))
      (else
        (goto _label_2)))))

(event Custom|DeactivatedDueToLandClaim
  ;[1 1 1] Landclaim deactivated the camp. Re-check once in a while to see if the camp can respawn
  (bind _returnvalue (Utilities|Time|SetTimerbyEvent (delegate Custom|DeactivatedDueToLandClaim_Inner) 3e+02))
  (Variables|Default|SetDeactivatedLandClaimTimer _returnvalue))

(event Custom|InitCamp
  ;[1 1 1] Figure out if camp is active on init
  (bind _array_element (Utilities|Array|ForEachLoopwithBreak (Variables|Camps|GetCampActors) :!label _label)
    (:LoopBody
      (Utilities|IsValid _array_element
        (:Is%20Valid
          (bind _returnvalue (Class|LandClaimSystem|CanClaimSphere "Building" (Utilities|Struct|MakeClaimOwnershipParams (Class|UniqueID|MakeNullUID)) (Transformation|GetActorLocation _array_element) (Variables|Default|GetPlayerBuilt_Claim_Radius)))
          (if _returnvalue
            ;[1 1 1] Bind Destroyed event. Fill CampEssentials
            (Game|BindEventtoOnDestroyed _array_element (delegate Custom|Camper_Destroyed))
            (if (Utilities|DoesObjectImplementInterface _array_element "/Game/Systems/Camps/I_CampActorInterface.I_CampActorInterface_C")
              (bind _isessential (Class|ICampActorInterface|CheckIsCampEssential(Message) _array_element))
              (if _isessential
                (Utilities|Array|AddUnique (Variables|Camps|GetCampEssentials) _array_element)))
            (else
              (CallFunction|SetCampActiveState false "NewEnumerator2")
              (goto _label Break))))))
    (:Completed
      ;[1 1 1] If camp isn't active, kill the actors and start the timer that checks if the spawn can respawn periodically.
      (if (not (Variables|Camps|GetIsCampActive))
        (for _array_element_2 (Variables|Camps|GetCampActors)
          (Utilities|IsValid _array_element_2
            (:Is%20Valid
              (Utilities|Array|Add (Variables|Camps|GetDestroyedActors) (Utilities|Struct|MakeST_CampActor (Utilities|GetClass _array_element_2) (Transformation|GetActorTransform _array_element_2) 0.0))
              (Actor|DestroyActor _array_element_2))))
        (Utilities|Array|Clear (Variables|Camps|GetCampActors))
        (CallFunction|DeactivatedDuetoLandClaim)))))

(event Custom|DeactivatedDueToLandClaim_Inner
  ;[1 1 1] Landclaim deactivated the camp. Re-check once in a while to see if the camp can respawn
  (CallFunction|SetCampActiveState true "NewEnumerator1")
  (bind _array_element (Utilities|Array|ForEachLoopwithBreak (Variables|Camps|GetDestroyedActors) :!label _label)
    (:LoopBody
      (bind _returnvalue (Class|LandClaimSystem|CanClaimSphere "Building" (Utilities|Struct|MakeClaimOwnershipParams (Class|UniqueID|MakeNullUID)) (.Location (Math|Transform|BreakTransform (.Transform (Utilities|Struct|BreakST_CampActor _array_element)))) (Variables|Default|GetPlayerBuilt_Claim_Radius)))
      (if _returnvalue
        (bind _returnvalue_2 (Class|PlayerPawnRegistry|HasPawnWithinDistance (Variables|Camps|GetPlayerPawnRegistry) (.Location (Math|Transform|BreakTransform (.Transform (Utilities|Struct|BreakST_CampActor _array_element)))) (Variables|/Game/Systems/Camps/BP_CampSystemComponent.BP_CampSystemComponent_C|GetCampRespawnExclusionRadius (Variables|Camps|GetCampSystem))))
        (if _returnvalue_2
          (CallFunction|SetCampActiveState false "NewEnumerator5" :!label _label_2)
          (goto _label Break))
        (else
          (goto _label_2))))
    (:Completed
      (if (Variables|Camps|GetIsCampActive)
        (for _array_element_2 (Variables|Camps|GetDestroyedActors)
          (bind _spawnedactor (CallFunction|SpawnCampActor (.Class (Utilities|Struct|BreakST_CampActor _array_element_2)) (.Transform (Utilities|Struct|BreakST_CampActor _array_element_2))))
          (Game|BindEventtoOnDestroyed _spawnedactor (delegate Custom|Camper_Destroyed)))
        (else
          (CallFunction|DeactivatedDuetoLandClaim))))))

(event EventBeginPlay
  (bind _returnvalue (Game|GetGameMode))
  (bind _returnvalue_2 (Actor|GetComponentsByClass _returnvalue "/Game/Systems/Camps/BP_CampSystemComponent.BP_CampSystemComponent_C"))
  ;[1 1 1] BeginPlay, initialize and register camp with the CampSystem.
  (if (Networking|IsServer)
    (for _array_element (Variables|Camps|GetCampActors)
      (Utilities|IsValid _array_element
        (:Is%20Valid
          (Utilities|Array|Add (Variables|Camps|GetCampActorData) (Utilities|Struct|MakeST_CampActor (Utilities|GetClass _array_element) (Transformation|GetActorTransform _array_element) 0.0))
          (if (Utilities|DoesObjectImplementInterface _array_element "/Game/Systems/Camps/I_CampActorInterface.I_CampActorInterface_C")
            (bind _isessential (Class|ICampActorInterface|CheckIsCampEssential(Message) _array_element))
            (if _isessential
              (Variables|Camps|SetHasCampEssentials true))))))
    (if (> (Utilities|Array|Length _returnvalue_2) 0) :!label _label
      (bind _output_get (Variables|Camps|SetCampSystem (Utilities|Array|Get(acopy) _returnvalue_2)))
      (Default|RegisterCamp _output_get self)
      (bind _outactors (Actor|GetAllActorsOfClass "/Script/ConanSandbox.ConanWorldSettings"))
      (bind _returnvalue_3 (Class|ConanWorldSettings|GetPlayerPawnRegistry (Utilities|Array|Get(acopy) _outactors)))
      (Variables|Camps|SetPlayerPawnRegistry _returnvalue_3)
      (elif (<= (Variables|Default|GetRetryRegistrationCounter) 5)
        (Class|LoggerLibrary|DWLogString (Utilities|String|Append "Didn't find CampSystemComponent, retrying in a few seconds. Attempt " (Utilities|String|ToString(Integer) (Variables|Default|GetRetryRegistrationCounter)) " of 5") "NPC" "INFOL_DATAWARNING")
        (Utilities|FlowControl|Delay 4.0)
        (Math|Integer|IncrementInt (Variables|Default|GetRetryRegistrationCounter)
          (:%20%20
            (goto _label)))
        (else
          (Class|LoggerLibrary|DWLogString "Couldn't register camp! Giving up, this camp is now broken and will be disabled." "NPC" "INFOL_CODEERROR")
          (CallFunction|SetCampActiveState false "NewEnumerator4")
          (for _array_element_2 (Variables|Camps|GetCampActors)
            (Actor|DestroyActor _array_element_2)))))))

(event EventAddTerritorySpawnerReference
  (params (TerritorySpawner :type Actor%20Object%20Reference))
  (Utilities|Array|AddUnique (Variables|Default|GetTerritorySpawners) TerritorySpawner))

(fn UpdateCachedWaypointsandSpawnPoints
  (if (Variables|Cache|GetIsSpawnPointAndWaypointCacheValid?)
    (return)
    (else
      (Utilities|Array|Clear (Variables|Cache|GetCachedSpawnPoints))
      (Utilities|Array|Clear (Variables|Cache|GetCachedWaypoints))
      (for _array_element (Variables|Camps|GetCampActors)
        (bind _asstatic_spawn_point (Utilities|Casting|CastToStaticSpawnPoint _array_element)
          (:then
            (Utilities|Array|AddUnique (Variables|Cache|GetCachedSpawnPoints) _asstatic_spawn_point))
          (:CastFailed
            (bind _asstatic_waypoint (Utilities|Casting|CastToStaticWaypoint _array_element))
            (Utilities|Array|AddUnique (Variables|Cache|GetCachedWaypoints) _asstatic_waypoint))))
      (Variables|Cache|SetIsSpawnPointAndWaypointCacheValid? true)
      (return))))

(fn SpawnCampActor
  (params (Class :type Actor%20Class%20Reference) (Transform :type Transform))
  (bind _returnvalue (Game|SpawnActorfromClass Class Transform "Undefined" 0 0))
  (Utilities|Array|Add (Variables|Camps|GetCampActors) _returnvalue)
  (if (Utilities|DoesObjectImplementInterface _returnvalue "/Game/Systems/Camps/I_CampActorInterface.I_CampActorInterface_C")
    (bind _isessential (Class|ICampActorInterface|CheckIsCampEssential(Message) _returnvalue))
    (if _isessential
      (Utilities|Array|AddUnique (Variables|Camps|GetCampEssentials) _returnvalue)
      (return _returnvalue)
      (else
        _)))
  (return 0))

(fn SetCampActiveState
  (params (IsActive :type Boolean) (State :type ST_CampDebugStates%20Enum))
  (Variables|Camps|SetIsCampActive IsActive)
  (if (Utilities|Enum|NotEqual(Enum) State (Variables|Default|GetDebugState))
    (Variables|Default|SetDebugState State)))

(fn GetDebugState
  (return (Utilities|String|EnumtoString (Variables|Default|GetDebugState))))

(fn GetDebugString
  (bind _respawningactors (Variables|Camps|GetRespawningActors))
  (bind _destroyedactors (Variables|Camps|GetDestroyedActors))
  (bind _returnvalue (Utilities|Array|Length _destroyedactors))
  (bind _returnvalue_2 (Utilities|Array|Length _respawningactors))
  (CallFunction|UpdateCachedWaypointsandSpawnPoints)
  (bind _currentstate (CallFunction|GetDebugState))
  (return (Utilities|String|Append "State: " _currentstate " 
NumActors: " (Utilities|String|ToString(Integer) (+ (Utilities|Array|Length (Variables|Camps|GetCampActors)) _returnvalue _returnvalue_2)) " 
NumEssentials: " (Utilities|String|ToString(Integer) (Utilities|Array|Length (Variables|Camps|GetCampEssentials))) " 
NumRespawning: " (Utilities|String|ToString(Integer) _returnvalue_2) " 
NumDestroyed: " (Utilities|String|ToString(Integer) _returnvalue) " 
NumSpawnPoints:" (Utilities|String|ToString(Integer) (Utilities|Array|Length (Variables|Cache|GetCachedSpawnPoints))) " 
NumWaypoints:" (Utilities|String|ToString(Integer) (Utilities|Array|Length (Variables|Cache|GetCachedWaypoints))) (select (Math|Boolean|ORBoolean (Utilities|Enum|Equal(Enum) (Variables|Default|GetDebugState) "NewEnumerator2") (Utilities|Enum|Equal(Enum) (Variables|Default|GetDebugState) "NewEnumerator5") false) (Utilities|String|Append " 
LandClaim respawn timer remaining: " (Utilities|String|ToString(Float) (Utilities|Time|GetTimerRemainingTimebyHandle (Variables|Default|GetDeactivatedLandClaimTimer)))) ""))))

(fn GetDebugStringNPCs
  (for (_array_element _array_index) (Variables|Cache|GetCachedSpawnPoints)
    (bind _asbp_manual_spawn_point (Utilities|Casting|CastToBP_ManualSpawnPoint _array_element))
    (LocalVariables|SetnpcDebugInfo (Utilities|String|Append (LocalVariables|GetnpcDebugInfo) " 
  " (Utilities|String|Append "  #" (Utilities|String|ToString(Integer) _array_index) " " (Utilities|GetDisplayName _array_element)) " Human NPCs: " (Utilities|String|ToString(Integer) (Utilities|Array|Length (Variables|/Game/Systems/AI/Navigation/BP_ManualSpawnPoint.BP_ManualSpawnPoint_C|GetHumanOptions _asbp_manual_spawn_point))) " Wildlife NPCs: " (Utilities|String|ToString(Integer) (Utilities|Array|Length (Variables|/Game/Systems/AI/Navigation/BP_ManualSpawnPoint.BP_ManualSpawnPoint_C|GetWildlifeOptions _asbp_manual_spawn_point))) " Alive: " (Utilities|String|ToString(Boolean) (and (Variables|/Game/Systems/AI/Navigation/BP_ManualSpawnPoint.BP_ManualSpawnPoint_C|GetHasSpawned _asbp_manual_spawn_point) (not (Variables|/Game/Systems/AI/Navigation/BP_ManualSpawnPoint.BP_ManualSpawnPoint_C|GetWaitingForRespawn _asbp_manual_spawn_point)))) " Respawning: " (Utilities|String|ToString(Boolean) (Variables|/Game/Systems/AI/Navigation/BP_ManualSpawnPoint.BP_ManualSpawnPoint_C|GetWaitingForRespawn _asbp_manual_spawn_point)) (select (Utilities|Time|IsTimerActivebyHandle (Variables|/Game/Systems/AI/Navigation/BP_ManualSpawnPoint.BP_ManualSpawnPoint_C|GetRespawnTimerHandle _asbp_manual_spawn_point)) (Utilities|String|Append " Remaining respawn time: " (Utilities|String|ToString(Float) (Utilities|Time|GetTimerRemainingTimebyHandle (Variables|/Game/Systems/AI/Navigation/BP_ManualSpawnPoint.BP_ManualSpawnPoint_C|GetRespawnTimerHandle _asbp_manual_spawn_point))) " of " (Utilities|String|ToString(Float) (* (Variables|/Game/Systems/AI/Navigation/BP_ManualSpawnPoint.BP_ManualSpawnPoint_C|GetRespawnTimer _asbp_manual_spawn_point) (Variables|/Game/Systems/BP_ServerSettings.BP_ServerSettings_C|GetNPCRespawnMultiplier (|GetServerSettings))))) " Not respawning"))))
  (LocalVariables|SetnpcDebugInfo (Utilities|String|Append (LocalVariables|GetnpcDebugInfo) " 
TerritorySpawners: "))
  (for (_array_element_2 _array_index_2) (Variables|Default|GetTerritorySpawners)
    (LocalVariables|SetnpcDebugInfo (Utilities|String|Append (LocalVariables|GetnpcDebugInfo) " 
  #" (Utilities|String|ToString(Integer) _array_index_2) " " (Utilities|GetDisplayName _array_element_2))))
  (return (Utilities|String|Append "Num spawn points: " (Utilities|String|ToString(Integer) (Utilities|Array|Length (Variables|Cache|GetCachedSpawnPoints))) (LocalVariables|GetnpcDebugInfo))))

(fn GetSpawnPoints
  (CallFunction|UpdateCachedWaypointsandSpawnPoints)
  (return (Variables|Cache|GetCachedSpawnPoints)))

(fn GetWaypoints
  (CallFunction|UpdateCachedWaypointsandSpawnPoints)
  (return (Variables|Cache|GetCachedWaypoints)))

(fn IsStaticNavigationProviderActive
  (if (Variables|Camps|GetForceCampActive)
    (return true)
    (else
      (return (and (Variables|Camps|GetIsCampActive) (or (not (Variables|Camps|GetHasCampEssentials)) (> (Utilities|Array|Length (Variables|Camps|GetCampEssentials)) 0)))))))