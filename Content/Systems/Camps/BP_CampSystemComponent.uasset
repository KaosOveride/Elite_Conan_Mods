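; Camp system component that picks a random camp layer at BeginPlay to decide which registered camps are live for the session.
; Once both BeginPlay and loading are done, it initializes camps with a matching or empty layer list, and deactivates the others and destroys their actors.
; A DebugCamps command returns text reports: camp lists filtered by radius or state, single-camp details, or spawner probability groups.
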(event EventBeginPlay
  (Variables|Camps|SetCurrentCampLayer (Math|Random|RandomIntegerinRange 0 (Variables|Camps|Settings|GetMaxCampLayer)))
  (Variables|Default|SetHasBegunPlay true)
  (if (Variables|Default|GetLoadingIsDone)
    (for _array_element (Variables|Camps|GetRegisteredCamps)
      (CallFunction|ProcessCamp _array_element))))

(fn RegisterCamp
  (params (Camp :type BP%20Camp%20Component%20Object%20Reference))
  (Utilities|Array|AddUnique (Variables|Camps|GetRegisteredCamps) Camp)
  (if (and (Variables|Default|GetHasBegunPlay) (Variables|Default|GetLoadingIsDone))
    (CallFunction|ProcessCamp Camp)))

(fn ProcessCamp
  (params (Camp :type BP%20Camp%20Component%20Object%20Reference))
  (bind _camplayer (Variables|/Game/Systems/Camps/BP_CampComponent.BP_CampComponent_C|GetCampLayer Camp))
  (if (> (Utilities|Array|Length _camplayer) 0)
    (if (!= (Utilities|Array|FindItem _camplayer (Variables|Camps|GetCurrentCampLayer)) -1)
      (Default|InitCamp Camp :!label _label)
      (else
        (Default|SetCampActiveState Camp false "NewEnumerator6")
        (for _array_element (Variables|/Game/Systems/Camps/BP_CampComponent.BP_CampComponent_C|GetCampActors Camp)
          (Actor|DestroyActor _array_element))))
    (else
      (goto _label))))

(fn LoadingDone
  (Variables|Default|SetLoadingIsDone true)
  (if (Variables|Default|GetHasBegunPlay)
    (for _array_element (Variables|Camps|GetRegisteredCamps)
      (CallFunction|ProcessCamp _array_element))))

(fn DebugCamps
  (params (Args :type String) (Controller :type Conan%20Player%20Controller%20Object%20Reference))
  (LocalVariables|SetlocalArgs Args)
  (LocalVariables|SetPrintList (Class|GameplayStatics|HasOption Args "List"))
  (LocalVariables|SetHasRadius (Class|GameplayStatics|HasOption Args "Radius"))
  (LocalVariables|SetRadius (Math|Conversions|ToFloat(Integer) (Class|GameplayStatics|ParseOption Args "Radius")))
  (bind _output_get (LocalVariables|SetHasState (Class|GameplayStatics|HasOption Args "State")))
  (if _output_get
    ;[1 1 1] Process TargetState
    (bind _enumvalue (|ForEachST_CampDebugStates)
      (:LoopBody
        (if (Utilities|Enum|Equal(Enum) (Class|GameplayStatics|ParseOption (LocalVariables|GetlocalArgs) "State") (Utilities|String|EnumtoString _enumvalue))
          (LocalVariables|SetTargetState _enumvalue)
          (LocalVariables|SetFoundState true)))
      (:then
        (if (LocalVariables|GetFoundState)
          (bind _outactors (Actor|GetAllActorsOfClass "/Game/Systems/Camps/BP_CampOwner.BP_CampOwner_C" :!label _label))
          ;[1 1 1] Filter Radius
          (if (LocalVariables|GetHasRadius)
            (for _array_element _outactors
              (if (<= (Transformation|GetSquaredDistanceTo _array_element (Pawn|GetControlledPawn Controller)) (Math|Float|Square (LocalVariables|GetRadius)))
                (Utilities|Array|Add (LocalVariables|GetCampOwners) _array_element)))
            (else
              (LocalVariables|SetCampOwners _outactors)))
          ;[1 1 1] Filter TargetState
          (if (LocalVariables|GetHasState)
            (for _array_element_2 (LocalVariables|GetCampOwners)
              (if (Utilities|Enum|Equal(Enum) (Variables|/Game/Systems/Camps/BP_CampComponent.BP_CampComponent_C|GetDebugState (Variables|/Game/Systems/Camps/BP_CampOwner.BP_CampOwner_C|GetBP_CampComponent _array_element_2)) (LocalVariables|GetTargetState))
                (Utilities|Array|Add (LocalVariables|GettempCampOwners) _array_element_2)))
            (LocalVariables|SetCampOwners (LocalVariables|GettempCampOwners)))
          ;[1 1 1] Print List of camps
          (if (LocalVariables|GetPrintList)
            (LocalVariables|SetlocalDebugMessage (Utilities|String|Append (select (LocalVariables|GetHasRadius) (Utilities|String|Append "Camps within Radius " (Utilities|String|ToString(Float) (LocalVariables|GetRadius)) ", State: ") "All Camps, State: ") (select (LocalVariables|GetHasState) (Utilities|String|EnumtoString (LocalVariables|GetTargetState)) "All") " Num: " (Utilities|String|ToString(Integer) (Utilities|Array|Length (LocalVariables|GetCampOwners)))))
            (for (_array_element_3 _array_index) (LocalVariables|GetCampOwners)
              (bind _currentstate (Default|GetDebugState (Variables|/Game/Systems/Camps/BP_CampOwner.BP_CampOwner_C|GetBP_CampComponent _array_element_3)))
              (LocalVariables|SetlocalDebugMessage (Utilities|String|Append (LocalVariables|GetlocalDebugMessage) " 
#" (Utilities|String|ToString(Integer) _array_index) " " (Utilities|GetDisplayName _array_element_3) " " _currentstate)))
            (return (LocalVariables|GetlocalDebugMessage))
            (else
              ;[1 1 1] Print Target Info
              (if (Class|GameplayStatics|HasOption (LocalVariables|GetlocalArgs) "Target")
                (for _array_element_4 (LocalVariables|GetCampOwners)
                  (if (Utilities|Enum|Equal(Enum) (Utilities|GetDisplayName _array_element_4) (Class|GameplayStatics|ParseOption (LocalVariables|GetlocalArgs) "Target"))
                    (bind _string (Default|GetDebugString (Variables|/Game/Systems/Camps/BP_CampOwner.BP_CampOwner_C|GetBP_CampComponent _array_element_4)))
                    (bind _debugstring (Default|GetDebugStringNPCs (Variables|/Game/Systems/Camps/BP_CampOwner.BP_CampOwner_C|GetBP_CampComponent _array_element_4)))
                    (LocalVariables|SetlocalDebugMessage (Utilities|String|Append (Utilities|GetDisplayName _array_element_4) " Debug Info: 
" _string " 
" _debugstring))))
                (return (LocalVariables|GetlocalDebugMessage))
                (else
                  ;[1 1 1] Spawner Probability Groups
                  (if (Class|GameplayStatics|HasOption (LocalVariables|GetlocalArgs) "Groups")
                    (LocalVariables|SetlocalDebugMessage "Spawner Groups: 
 Bands(Not sorted):")
                    (for (_array_element_5 _array_index_2) (Class|ConanWorldSettings|GetSpawnProbabilityBandsBPCopy (Class|FuncomGenericLibrary|GetWorldSettings))
                      (LocalVariables|SetlocalDebugMessage (Utilities|String|Append (LocalVariables|GetlocalDebugMessage) " 
  #" (Utilities|String|ToString(Integer) _array_index_2) " Radius: " (Utilities|String|ToString(Float) (.radius _array_element_5)) " Weight: " (Utilities|String|ToString(Integer) (.weight _array_element_5)))))
                    (for (_array_element_6 _array_index_3) (Class|NPCRegistry|DebugGetSpawnerProbabilityGroups)
                      (LocalVariables|SetlocalDebugMessage (Utilities|String|Append (LocalVariables|GetlocalDebugMessage) " 
 Group: #" (Utilities|String|ToString(Integer) _array_index_3) " Normalized Weight: " (Utilities|String|ToString(Float) (.NormalizedWeight (Utilities|Struct|BreakDebugSpawnProbabilityGroup _array_element_6))) " Actual Weight: " (Utilities|String|ToString(Integer) (.ActualWeight (Utilities|Struct|BreakDebugSpawnProbabilityGroup _array_element_6)))))
                      (for (_array_element_7 _array_index_4) (.Members (Utilities|Struct|BreakDebugSpawnProbabilityGroup _array_element_6))
                        (bind _asnpcterritory_spawner (Utilities|Casting|CastToNPCTerritorySpawner _array_element_7))
                        (LocalVariables|SetlocalDebugMessage (Utilities|String|Append (LocalVariables|GetlocalDebugMessage) " 
    #" (Utilities|String|ToString(Integer) _array_index_4) " " (Utilities|GetDisplayName _asnpcterritory_spawner)))))
                    (return (LocalVariables|GetlocalDebugMessage))
                    (else
                      (return "Available options are: 
?List                                     - Prints a list of relevant camp actors 
?State=<some state>      - Limits relevant actors to State of choosing 
?Radius=<radius>            - Limits relevant actors to within radius from caller 
?Target=<Actor Name>  - Prints specific information about target camp 
?Groups                              - Prints list of spawners and which probability group they are in.")))))))
          (else
            (bind _enumvalue_2 (|ForEachST_CampDebugStates)
              (:LoopBody
                (LocalVariables|SetlocalDebugMessage (Utilities|String|Append (LocalVariables|GetlocalDebugMessage) " 
" (Utilities|String|EnumtoString _enumvalue_2))))
              (:then
                (return (Utilities|String|Append "Unknown target state: " (Class|GameplayStatics|ParseOption (LocalVariables|GetlocalArgs) "State") " 
Allowed states are:" (LocalVariables|GetlocalDebugMessage)))))))))
    (else
      (goto _label))))