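; Admin-only helper that spawns NPCs for the control panel a short distance in front of the player.
; Named rows resolve against the NPC list table, then the zoo table, and spawn with optional aggression override.
; Spawn-table rows can instead be instantly thrallified, replacing the NPC with a converted thrall item in the player's backpack.
; NPCs left in the world join the spawned list, and "Human-" row prefixes flag human NPCs.
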(fn SpawnNPCfromControlPanel
  (params (PlayerCharacter :type Actor%20Object%20Reference) (SpawnedNPCList :type Array%20of%20Pawn%20Object%20References) (SetAggression :type Boolean) (AggressionValue :type Aggression%20Enum) (RowName :type Name) (HumanType :type NPCHumans%20Enum) (IsSpawnTable :type Boolean) (InstantThrallify :type Boolean))
  (bind _returnvalue (Transformation|GetActorTransform PlayerCharacter))
  (bind _returnvalue_2 (Math|Vector|GetForwardVector (.rotation _returnvalue)))
  (bind _returnvalue_3 (* _returnvalue_2 350))
  (bind _returnvalue_4 (+ (.location _returnvalue) _returnvalue_3))
  (bind _asconan_character (Utilities|Casting|CastToConanCharacter PlayerCharacter)
    (:then
      (LocalVariables|SetPlayer _asconan_character)
      (bind _asconan_player_controller (Utilities|Casting|CastToConanPlayerController (Pawn|GetController _asconan_character))
        (:then
          (if (Class|ConanPlayerController|IsAdmin _asconan_player_controller)
            (if (not IsSpawnTable)
              (bind _returnvalue_5 (Utilities|GetDataTableRow "/Game/Systems/Spawning/NPCList_Table.NPCList_Table" RowName)
                (:then
                  (LocalVariables|SetNPCEntry _returnvalue_5))
                (:RowNotFound
                  (bind _returnvalue_6 (Utilities|GetDataTableRow "/Game/Systems/Spawning/NPCList_Zoo_Table.NPCList_Zoo_Table" RowName)
                    (:then
                      (LocalVariables|SetNPCEntry _returnvalue_6))
                    (:RowNotFound
                      (Utilities|DebugPrint "NPC entry not found in tables!" "INFOL_DATAERROR" "AI" true "(R=1.000000,G=0.000000,B=0.000000,A=1.000000)" 5.0
                        (:Output
                          (return)))))))
              (bind (_success _npc) (CallFunction|TrySpawnNPCLowLevel (.behavior_tree (LocalVariables|GetNPCEntry)) (- (.Yaw (Math|Rotator|BreakRotator (.rotation _returnvalue))) 1.8e+02) (.npc (LocalVariables|GetNPCEntry)) (.controller (LocalVariables|GetNPCEntry)) _returnvalue_4 1e+04 (Utilities|String|Append "Spawning " (Utilities|String|ToString(Name) RowName) " from control panel") 0 "" false HumanType (CallFunction|IsHumanRowName RowName) 0 0 0 0 0 (.name (LocalVariables|GetNPCEntry))))
              (if _success
                (Utilities|Array|Add SpawnedNPCList _npc)
                (if SetAggression
                  (bind _asbase_npc (Utilities|Casting|CastToBaseNPC _npc)
                    (:then
                      (Variables|/Game/Characters/BaseNPC.BaseNPC_C|SetAggression _asbase_npc AggressionValue))
                    (:CastFailed
                      _)))
                (else
                  (Utilities|DebugPrint "NPC spawn failed! See logs for details." "INFOL_DATAERROR" "AI" true "(R=1.000000,G=0.000000,B=0.000000,A=1.000000)" 5.0
                    (:Output
                      _))))
              (return)
              (else
                (bind (_success_2 _npc_2 _characterlayout) (CallFunction|TrySpawnNPCfromSpawnTableLowLevel RowName false _returnvalue_4 1e+04))
                (if _success_2
                  (if InstantThrallify
                    (bind _asconan_character_2 (Utilities|Casting|CastToConanCharacter _npc_2)
                      (:then
                        (bind _returnvalue_7 (Class|GameItemSpawner|SpawnThrallItem 0 "/Script/ConanSandbox.ThrallItem" _asconan_character_2 _characterlayout))
                        (Utilities|IsValid _returnvalue_7
                          (:Is%20Valid
                            (Actor|DestroyActor _asconan_character_2)
                            (Class|GameItem|SetIntStat _returnvalue_7 "ThrallIsConverted" 1 false)
                            (bind _returnvalue_8 (Class|ConanCharacter|GetBackpackInventory (LocalVariables|GetPlayer)))
                            (Class|ItemInventory|AddItem _returnvalue_8 _returnvalue_7 -1 0 -1))
                          (:Is%20Not%20Valid
                            (Utilities|Array|Add SpawnedNPCList _npc_2 :!label _label)
                            (return))))
                      (:CastFailed
                        (goto _label)))
                    (else
                      (goto _label))))))
            (else
              (return))))
        (:CastFailed
          (return))))
    (:CastFailed
      (return))))

(fn IsHumanRowName
  (params (RowName :type Name))
  (return (Utilities|String|StartsWith (Utilities|String|ToString(Name) RowName) "Human-" "CaseSensitive")))