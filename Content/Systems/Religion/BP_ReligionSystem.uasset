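; Religion function library that tracks each character's favor with the gods in the Favors array of its ReligionData component.
; Crafting looks up the recipe's per-god favor grant in a data table, defaulting to zeros, and passes it to ModifyFavor.
; ModifyFavor sets Mitra (index 4) against the others: Mitra's gain lowers every other god, and their summed gains lower Mitra.
; Helpers add favor by god and log totals; AdjustFavor is empty.
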(fn AddFavorbyGod
  (params (Modify%20By :type Float%20%28single-precision%29) (God :type Gods%20Enum) (Character :type Base%20BP%20Combat%20Object%20Reference))
  (bind _returnvalue (Actor|GetComponentsByClass Character "/Game/Systems/Religion/ReligionData.ReligionData_C"))
  (bind _returnvalue_2 (Math|Conversions|ToInteger(Byte) God))
  (bind _item (Utilities|Array|Get(acopy) _returnvalue))
  (bind _favors (Variables|/Game/Systems/Religion/ReligionData.ReligionData_C|GetFavors _item))
  (LocalVariables|SetFavor%20Array _favors)
  (if (> _returnvalue_2 (Utilities|Array|Length (LocalVariables|GetFavor%20Array)))
    (Utilities|Array|AddUnique (LocalVariables|GetFavor%20Array) Modify%20By)
    (else
      (Utilities|Array|SetArrayElem _favors _returnvalue_2 (+ Modify%20By (Utilities|Array|Get(acopy) (LocalVariables|GetFavor%20Array) _returnvalue_2))))))

(fn PrintFavor
  (params (Target :type Base%20BP%20Combat%20Object%20Reference))
  (LocalVariables|SetPrint%20Output "Favor change (")
  (for (_array_element _array_index) (Variables|/Game/Systems/Religion/ReligionData.ReligionData_C|GetFavors (Utilities|Array|Get(acopy) (Actor|GetComponentsByClass Target "/Game/Systems/Religion/ReligionData.ReligionData_C")))
    (LocalVariables|SetPrint%20Output (Utilities|String|Append (LocalVariables|GetPrint%20Output) (Utilities|String|ToString(Text) (Utilities|Text|FormatText "{God} = {Favor}" (Utilities|Text|ToText(String) (Utilities|String|EnumtoString (Utilities|Enum|ByteToEnumGods (Math|Conversions|ToByte(Integer) _array_index)))) (Utilities|Text|ToText(Float) _array_element "HalfToEven"))) ", ")))
  (Class|LoggerLibrary|DWLogString 0 (Utilities|String|Append (LocalVariables|GetPrint%20Output) ")") "ItemInventory" "INFOL_IMPORTANT" true))

(fn AdjustFavor
  (params (Character :type Base%20BP%20Combat%20Object%20Reference) (Victim%20Favor :type Array%20of%20Floats%20%28single-precision%29) (Modify%20By%20Override :type Float%20%28single-precision%29)))

(fn HandleFavorfromCrafting
  (params (Recipe%20ID :type Game%20Item%20Object%20Reference) (Character :type Base%20Player%20Char%20Object%20Reference))
  ;[1 1 1] Determine if recipe should give favor and how much
  (bind _favors (CallFunction|CalculateFavorfromRecipeID (Variables|/Script/ConanSandbox.GameItem|GetTemplateID Recipe%20ID) Character))
  ;[1 1 1] Handle Favor Interactions
  (CallFunction|ModifyFavor _favors Character Character))

(fn CalculateFavorfromRecipeID
  (params (Template%20ID :type Integer))
  (bind _returnvalue (Utilities|String|ToString(Integer) Template%20ID))
  (bind _returnvalue_2 (Utilities|String|StringToName _returnvalue))
  (bind _outrownames (DataTable|GetDataTableRowNames "/Game/Systems/Religion/FavorFromRecipeTable.FavorFromRecipeTable"))
  ;[1 1 1] Does the row exist?
  (if (!= (Utilities|Array|FindItem _outrownames _returnvalue_2) -1)
    (bind _returnvalue_3 (Utilities|GetDataTableRow "/Game/Systems/Religion/FavorFromRecipeTable.FavorFromRecipeTable" _returnvalue_2)
      (:then
        (return (.favorgranted _returnvalue_3)))
      (:RowNotFound
        _)))
  (return (Utilities|Array|MakeArray 0.0 0.0 0.0 0.0 0.0 0.0 0.0 0.0)))

(fn ModifyFavor
  (params (Modify :type Array%20of%20Floats%20%28single-precision%29) (Character :type Base%20Player%20Char%20Object%20Reference))
  (bind _religiondata (Variables|/Game/Characters/BaseBPCombat.BaseBPCombat_C|GetReligionData Character))
  (bind _favors (Variables|/Game/Systems/Religion/ReligionData.ReligionData_C|GetFavors _religiondata))
  ;[1 1 1] Process Mitra vs Others
  (LocalVariables|SetMitra%20Favor 0.0)
  (LocalVariables|SetNon%20Mitra%20Favor 0.0)
  (for (_array_element _array_index) Modify
    ;;[1 1 1] If Mitra
    (if (== _array_index 4)
      (LocalVariables|SetMitra%20Favor _array_element)
      (else
        (LocalVariables|SetNon%20Mitra%20Favor (+ (LocalVariables|GetNon%20Mitra%20Favor) _array_element)))))
  (for (_array_element_2 _array_index_2) Modify
    ;[1 1 1] Mitra affects other favors and viceversa
    (if (== _array_index_2 4)
      (Utilities|Array|SetArrayElem _favors _array_index_2 (- (+ _array_element_2 (Utilities|Array|Get(acopy) _favors _array_index_2)) (LocalVariables|GetNon%20Mitra%20Favor)))
      (else
        (Utilities|Array|SetArrayElem _favors _array_index_2 (- (+ _array_element_2 (Utilities|Array|Get(acopy) _favors _array_index_2)) (LocalVariables|GetMitra%20Favor))))))
  (return))