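; Player camera manager that handles NVIDIA Ansel photo mode, constraining the free camera and managing player head visibility.
; Sessions disable player input and enable collision on a spawned BP_AnselCamera, then restore input and head state afterwards.
; Camera modify moves that proxy, reverting when it blocks movement or exceeds max height, otherwise clamping distance from origin.
; It reveals the head past a squared-distance threshold and pins the camera during cinematics via a console variable.
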(event EventOnPhotographySessionStart
  (bind _returnvalue (Game|GetPlayerCharacter 0))
  (|CallParentFunction)
  (Input|DisableInput _returnvalue (Game|Player|GetOwningPlayerController))
  (bind _asbase_player_char (Utilities|Casting|CastToBasePlayerChar _returnvalue))
  (bind _output_get (Variables|Default|SetBasePlayerChar _asbase_player_char))
  (Variables|Default|SetHeadVisibleBeforeAnselSession (Variables|/Game/Characters/BasePlayerChar.BasePlayerChar_C|GetHeadVisible _output_get))
  (Collision|SetActorEnableCollision (Variables|Default|GetAnselCamera) true))

(event EventOnPhotographySessionEnd
  (bind _baseplayerchar (Variables|Default|GetBasePlayerChar))
  (|CallParentFunction)
  (Input|EnableInput _baseplayerchar (Game|Player|GetOwningPlayerController))
  (Default|UpdateHeadVisibility _baseplayerchar (Variables|/Game/Characters/BasePlayerChar.BasePlayerChar_C|GetHeadVisible _baseplayerchar) (Variables|Default|GetHeadVisibleBeforeAnselSession))
  (Collision|SetActorEnableCollision (Variables|Default|GetAnselCamera) false))

(event EventBeginPlay
  (bind _returnvalue (Game|SpawnActorfromClass "/Game/Systems/BP_AnselCamera.BP_AnselCamera_C" (Math|Transform|MakeTransform "0, 0, 0" "0, 0, 0" "1,1,1") "Undefined" 0 0))
  (bind _output_get (Variables|Default|SetAnselCamera _returnvalue))
  (Collision|SetActorEnableCollision _output_get false))

(fn ConstructionScript)

(fn PhotographyCameraModify
  (params (NewCameraLocation :type Vector) (PreviousCameraLocation :type Vector) (OriginalCameraLocation :type Vector))
  (bind _baseplayerchar (Variables|Default|GetBasePlayerChar))
  (bind _baseplayerchar_2 (Variables|Default|GetBasePlayerChar))
  (bind _headvisible (Variables|/Game/Characters/BasePlayerChar.BasePlayerChar_C|GetHeadVisible _baseplayerchar))
  (LocalVariables|SetNewCamLocation NewCameraLocation)
  (LocalVariables|SetPreviousCamLocation PreviousCameraLocation)
  (LocalVariables|SetOriginalCamLocation OriginalCameraLocation)
  (if _headvisible
    _
    (else
      ;[1 1 1] Turn the head on when we are a certain distance from the starting point
      (if (and (not _headvisible) (> (Math|Vector|VectorLengthSquared (- (LocalVariables|GetNewCamLocation) (LocalVariables|GetOriginalCamLocation))) (Variables|Default|GetDistanceToShowHead)))
        (Default|UpdateHeadVisibility _baseplayerchar_2 (Variables|/Game/Characters/BasePlayerChar.BasePlayerChar_C|GetHeadVisible _baseplayerchar_2) true))))
  (bind _outvalue (Class|TestUtils|ReadConsoleVariableInt "r.Photography.InCinematic"))
  (if (Math|Conversions|ToBoolean(Integer) _outvalue)
    (return (LocalVariables|GetOriginalCamLocation))
    (else
      (Transformation|SetActorLocation (Variables|Default|GetAnselCamera) (LocalVariables|GetNewCamLocation) false false)
      (if (Variables|/Game/Systems/BP_AnselCamera.BP_AnselCamera_C|GetShouldBlockMovement (Variables|Default|GetAnselCamera))
        _
        (elif (> (.Z (Math|Vector|BreakVector (LocalVariables|GetNewCamLocation))) (Variables|Default|GetMaxCameraHeight))
          _
          (else
            ;[1 1 1] Keep moving
            (return (+ (Math|Vector|ClampVectorSize (- (LocalVariables|GetNewCamLocation) (LocalVariables|GetOriginalCamLocation)) 0.0 (Variables|Default|GetMaxDistanceFromOrigin)) (LocalVariables|GetOriginalCamLocation))))))
      ;[1 1 1] Return to previous location
      (return (LocalVariables|GetPreviousCamLocation)))))