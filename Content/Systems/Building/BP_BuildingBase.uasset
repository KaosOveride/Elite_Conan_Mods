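; Base Blueprint for building pieces: validates and performs placement, toggles snap socket visibility and disables shape collision on non-brush pieces.
; CanBePlaced extends the parent check with a downward landscape trace (pillars exempt), blocker volumes, box-checker overlaps, required snapping and upgrade detection by overlapped mesh.
; PlaceOnSocket spawns a non-replicated temporary brush to test overlaps and derive the mesh transform, then swaps it for an AddModule instance, consuming resources on success.
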(event Custom|ServerPlaceOnSocket
  (params (Target%20Socket%20Index :type Integer) (Building%20Class :type BP%20Building%20Base%20Class%20Reference) (Building%20Socket%20Index :type Integer))
  (CallFunction|PlaceonSocket 0 (Math|Transform|MakeTransform "0, 0, 0"))
  (Class|WorldPersistenceComponent|SaveActor self))

(event EventEndPlay
  (params (EndPlayReason :type EEndPlayReason%20Enum :default "Destroyed")))

(event EventBeginPlay
  (bind _textrender (Variables|Default|GetTextRender))
  (Utilities|IsValid _textrender
    (:Is%20Valid
      (Rendering|Components|TextRender|SetText _textrender (Variables|Default|GetTextRenderText)))
    (:Is%20Not%20Valid
      _))
  (if (not (Variables|Default|GetIsABrush))
    (for _array_element (Actor|GetComponentsByClass "/Script/Engine.ShapeComponent")
      (Collision|SetCollisionEnabled _array_element "NoCollision"))))

(event EventActorBeginOverlap
  (params (OtherActor :type Actor%20Object%20Reference)))

(event EventTick
  (params (DeltaSeconds :type Float%20%28single-precision%29)))

(fn ConstructionScript)

(fn PlaceonSocket
  (params (Building%20Class :type Building%20Base%20Class%20Reference) (TargetTransform :type Transform) (OwnerSystem :type BP%20Build%20System%20V%202%20Object%20Reference))
  (bind _returnvalue (Components|GetOwner OwnerSystem))
  (bind (_location _rotation) (Math|Transform|BreakTransform TargetTransform))
  (bind _asconan_character (Utilities|Casting|CastToConanCharacter _returnvalue))
  (bind _asbp_building_base (Utilities|Casting|CastToBP_BuildingBaseClass Building%20Class)
    (:then
      (bind _returnvalue_2 (Class|ConanCharacter|GetPrioritizedUID _asconan_character))
      (bind _returnvalue_3 (Game|SpawnActorfromClass Building%20Class TargetTransform "AlwaysSpawn" 0 0 (LocalVariables|GetAnnoyingWorkAround) _returnvalue_2))
      (bind _asbp_building_base_2 (Utilities|Casting|CastToBP_BuildingBase _returnvalue_3)
        (:then
          (Networking|SetReplicates _asbp_building_base_2 false)
          (Variables|/Script/ConanSandbox.BuildableBase|SetIsABrush _asbp_building_base_2 true)
          (if (<= (Utilities|Array|Length (Collision|GetOverlappingActors _asbp_building_base_2 "/Script/ConanSandbox.BuildingBase" :!class /Script/Engine.Actor)) 0)
            _
            (else
              (bind _asbp_building_base_3 (Utilities|Casting|CastToBP_BuildingBase (Utilities|Array|Get(acopy) (Collision|GetOverlappingActors _asbp_building_base_2 "/Script/ConanSandbox.BuildingBase" :!class /Script/Engine.Actor)))
                (:then
                  (if (and (Variables|/Script/ConanSandbox.BuildingBase|GetIsABrush _asbp_building_base_3) (<= (Utilities|Array|Length (Collision|GetOverlappingActors _asbp_building_base_2 "/Script/ConanSandbox.BuildingBase" :!class /Script/Engine.Actor)) 1))
                    _
                    (else
                      (Development|PrintString (Utilities|String|ToString(Text) (Utilities|Text|FormatText "Can't place there, overlapping: {a}" (Utilities|Text|ToText(Integer) (Utilities|Array|Length (Collision|GetOverlappingActors _asbp_building_base_2 "/Script/ConanSandbox.BuildingBase" :!class /Script/Engine.Actor))))) :!label _label)
                      (Actor|DestroyActor _asbp_building_base_2)
                      (return))))
                (:CastFailed
                  (goto _label)))))
          (bind _canconsume (Default|CanConsumeResources OwnerSystem))
          (if _canconsume
            (bind _output_get (LocalVariables|SetLocalMeshTransform (Math|Transform|MakeTransform (+ _location (.Location (Math|Transform|BreakTransform (Transformation|GetRelativeTransform (Variables|/Script/ConanSandbox.BuildingBase|GetInstancedBuildingMesh _asbp_building_base_2)))) (Math|Vector|RotateVector (.Location (Math|Transform|BreakTransform (.OutInstanceTransform (Components|InstancedStaticMesh|GetInstanceTransform (Variables|/Script/ConanSandbox.BuildingBase|GetInstancedBuildingMesh _asbp_building_base_2) 0 false)))) (Math|Rotator|CombineRotators (.Rotation (Math|Transform|BreakTransform (.OutInstanceTransform (Components|InstancedStaticMesh|GetInstanceTransform (Variables|/Script/ConanSandbox.BuildingBase|GetInstancedBuildingMesh _asbp_building_base_2) 0 false)))) (Math|Rotator|CombineRotators (.Rotation (Math|Transform|BreakTransform (Transformation|GetRelativeTransform (Variables|/Script/ConanSandbox.BuildingBase|GetInstancedBuildingMesh _asbp_building_base_2)))) _rotation)))) (Math|Rotator|CombineRotators (.Rotation (Math|Transform|BreakTransform (.OutInstanceTransform (Components|InstancedStaticMesh|GetInstanceTransform (Variables|/Script/ConanSandbox.BuildingBase|GetInstancedBuildingMesh _asbp_building_base_2) 0 false)))) (Math|Rotator|CombineRotators (.Rotation (Math|Transform|BreakTransform (Transformation|GetRelativeTransform (Variables|/Script/ConanSandbox.BuildingBase|GetInstancedBuildingMesh _asbp_building_base_2)))) _rotation)) (* (.Scale (Math|Transform|BreakTransform (Transformation|GetRelativeTransform (Variables|/Script/ConanSandbox.BuildingBase|GetInstancedBuildingMesh _asbp_building_base_2)))) (.Scale (Math|Transform|BreakTransform (.OutInstanceTransform (Components|InstancedStaticMesh|GetInstanceTransform (Variables|/Script/ConanSandbox.BuildingBase|GetInstancedBuildingMesh _asbp_building_base_2) 0 false))))))))
            (Default|PlayPlacementSound OwnerSystem _asbp_building_base_2)
            (Actor|DestroyActor _asbp_building_base_2)
            (bind _returnvalue_4 (Class|ConanCharacter|GetPrioritizedUID _asconan_character))
            (bind _returnvalue_5 (Class|BuildingBase|AddModule _asbp_building_base TargetTransform _output_get (Utilities|Array|MakeArray) false _returnvalue_4))
            (if _returnvalue_5
              (Default|ConsumeResources OwnerSystem)
              (else
                (bind _asconan_player_controller (Utilities|Casting|CastToConanPlayerController (Pawn|GetController _asconan_character) :!label _label_2)
                  (:then
                    (Utilities|IsValid _asconan_player_controller
                      (:Is%20Valid
                        (Class|ConanPlayerController|ClientHUDShowNotification _asconan_player_controller "Failed to place building" false))
                      (:Is%20Not%20Valid
                        _)))
                  (:CastFailed
                    _))))
            (else
              (Development|PrintString "Couldn't consume resources.")
              (Actor|DestroyActor _asbp_building_base_2)
              (goto _label_2)))
          (Class|WorldPersistenceComponent|SaveActor self)
          (return))
        (:CastFailed
          (return))))
    (:CastFailed
      (return))))

(fn HideAllSockets
  (Development|SetHiddeninGame (Variables|Default|GetBuildSockets) true true))

(fn ShowSockets
  (params (SocketTypeToShow :type Enum_BuildingSocketTypes%20Enum))
  (bind _returnvalue (Game|Player|GetPlayerPawn 0))
  (bind _returnvalue_2 (Actor|GetComponentsByClass _returnvalue "/Script/ConanSandbox.BuildSystemComponent"))
  (if (> (Utilities|Array|Length _returnvalue_2) 0)
    (if (Variables|/Script/ConanSandbox.BuildSystemComponent|GetShowBuildingSockets (Utilities|Array|Get(acopy) _returnvalue_2))
      (Development|SetHiddeninGame (Variables|Default|GetBuildSockets) false true))))

(fn CanbePlaced
  (params (AttachTo :type Buildable%20Base%20Object%20Reference) (InstanceIndex :type Integer))
  (bind _returnvalue (Transformation|GetActorLocation))
  (bind _secondaryoverlapbuildingboxchecker (Variables|Default|GetSecondaryOverlapBuildingBoxChecker))
  (bind _instancedbuildingmesh (Variables|Default|GetInstancedBuildingMesh))
  (bind _secondaryoverlapplaceablesboxchecker (Variables|Default|GetSecondaryOverlapPlaceablesBoxChecker))
  (bind _overlappingbuildingstaticmeshes (LocalVariables|GetOverlappingBuildingStaticMeshes))
  (bind _overlapbuildingboxchecker (Variables|Default|GetOverlapBuildingBoxChecker))
  (bind _overlapplaceablesboxchecker (Variables|Default|GetOverlapPlaceablesBoxChecker))
  (bind _instancedbuildingmesh_2 (Variables|Default|GetInstancedBuildingMesh))
  (bind _overlappingactors (Collision|GetOverlappingActors _overlapbuildingboxchecker "/Game/Systems/Building/BuildingBlockerVolume.BuildingBlockerVolume_C" :!class /Script/Engine.PrimitiveComponent))
  (bind _staticmesh (Variables|/Script/Engine.StaticMeshComponent|GetStaticMesh _instancedbuildingmesh))
  (bind _returnvalue_2 (StaticMesh|GetBoundingBox _staticmesh))
  (bind _max (Utilities|Struct|BreakBox _returnvalue_2))
  (bind _z (Math|Vector|BreakVector _max))
  (bind _returnvalue_3 (* _z 0.5))
  (bind (_failedmessage _returnvalue_4) (|CallParentFunction AttachTo InstanceIndex))
  ;[1 1 1] Check if above ground
  (bind _outhits (Class|KismetSystemLibrary|BoxTraceMultiforObjects (+ (.Location (Math|Transform|BreakTransform (.OutInstanceTransform (Components|InstancedStaticMesh|GetInstanceTransform _instancedbuildingmesh 0 false)))) (Variables|/Script/Engine.SceneComponent|GetRelativeLocation _instancedbuildingmesh) (+ _returnvalue (Math|Conversions|ToVector(Float) _returnvalue_3))) (- _returnvalue "0, 0,1000000000.000000") (Math|Vector|MakeVector 16.0 16.0 _returnvalue_3) (Transformation|GetWorldRotation _instancedbuildingmesh) (Utilities|Array|MakeArray "ObjectTypeQuery1") false 0 "None" true))
  (for _array_element _outhits
    (if (or (== (Utilities|GetClass (.HitActor (Collision|BreakHitResult _array_element))) "/Script/Landscape.Landscape") (== (Utilities|GetClass (.HitActor (Collision|BreakHitResult _array_element))) "/Script/Landscape.LandscapeProxy"))
      (LocalVariables|SetAboveGround true)))
  (if (or (LocalVariables|GetAboveGround) (Variables|Default|GetIsPillar))
    ;[1 1 1] Force generate overlap events
    (Variables|/Script/Engine.PrimitiveComponent|SetbForceGenerateOverlapEvents (Variables|Default|GetOverlapBuildingBoxChecker) true)
    (Variables|/Script/Engine.PrimitiveComponent|SetbForceGenerateOverlapEvents (Variables|Default|GetInstancedBuildingMesh) true)
    (Variables|/Script/Engine.PrimitiveComponent|SetbForceGenerateOverlapEvents (Variables|Default|GetOverlapPlaceablesBoxChecker) false)
    (Class|FuncomGenericLibrary|UpdateOverlaps self)
    (if (> (Utilities|Array|Length _overlappingactors) 0)
      ;[1 1 1] If blocked by a BuilingBlockerVolume
      (bind _asbuilding_blocker_volume (Utilities|Casting|CastToBuildingBlockerVolume (Utilities|Array|Get(acopy) _overlappingactors))
        (:then
          (return (Utilities|String|ToString(Text) (Variables|/Game/Systems/Building/BuildingBlockerVolume.BuildingBlockerVolume_C|GetMessageToPlayer _asbuilding_blocker_volume)) "Fail"))
        (:CastFailed
          (return "Overlapping with BuildingBlockerVolume but failed cast to BuildingBlockerVolume. This should not happen." "Fail")))
      (else
        (LocalVariables|SetOverlappingActors (Collision|GetOverlappingActors _instancedbuildingmesh_2 "/Script/Engine.Character" :!class /Script/Engine.PrimitiveComponent))
        (Utilities|Array|AppendArray (LocalVariables|GetOverlappingActors) (Collision|GetOverlappingActors _instancedbuildingmesh_2 "/Script/Foliage.InstancedFoliageActor" :!class /Script/Engine.PrimitiveComponent))
        (Utilities|Array|AppendArray (LocalVariables|GetOverlappingActors) (Collision|GetOverlappingActors _instancedbuildingmesh_2 "/Script/ConanSandbox.ResourceActorBase" :!class /Script/Engine.PrimitiveComponent))
        (Utilities|Array|Clear (LocalVariables|GetOverlappingBuildingStaticMeshes))
        (LocalVariables|SetOverlappingComponents (Class|PrimitiveComponent|GetOverlappingComponents (Variables|Default|GetOverlapBuildingBoxChecker)))
        (if (Variables|Default|GetUseSecondaryOverlapBuildingBoxChecker)
          ;[1 1 1] Secondary Building Box Overlap
          (Variables|/Script/Engine.PrimitiveComponent|SetbForceGenerateOverlapEvents _secondaryoverlapbuildingboxchecker true)
          (Utilities|Array|AppendArray (LocalVariables|GetOverlappingComponents) (Class|PrimitiveComponent|GetOverlappingComponents _secondaryoverlapbuildingboxchecker)))
        (for _array_element_2 (LocalVariables|GetOverlappingComponents)
          (bind _asinstanced_static_mesh_component (Utilities|Casting|CastToInstancedStaticMeshComponent _array_element_2)
            (:then
              (if (and (not (Utilities|Array|ContainsItem (Variables|Default|GetIgnoreOverlappingTheseFoilageMeshes) (Variables|/Script/Engine.StaticMeshComponent|GetStaticMesh _asinstanced_static_mesh_component))) (not (Utilities|Array|ContainsItem (Variables|Default|GetIgnoreOverlappingTheseMeshes) (Variables|/Script/Engine.StaticMeshComponent|GetStaticMesh _asinstanced_static_mesh_component))))
                (bind _asbp_building_base (Utilities|Casting|CastToBP_BuildingBase (Components|GetOwner _asinstanced_static_mesh_component)))
                (if (not (Variables|/Script/ConanSandbox.BuildableBase|GetIsABrush _asbp_building_base))
                  (Utilities|Array|Add (LocalVariables|GetOverlappingBuildingStaticMeshes) (Variables|/Script/Engine.StaticMeshComponent|GetStaticMesh _asinstanced_static_mesh_component)))))
            (:CastFailed
              ;[1 1 1] Check for overlapping placeables
              (bind _asstatic_mesh_component (Utilities|Casting|CastToStaticMeshComponent _array_element_2))
              (if (and (not (Utilities|Array|ContainsItem (Variables|Default|GetIgnoreOverlappingTheseFoilageMeshes) (Variables|/Script/Engine.StaticMeshComponent|GetStaticMesh _asstatic_mesh_component))) (not (Utilities|Array|ContainsItem (Variables|Default|GetIgnoreOverlappingTheseMeshes) (Variables|/Script/Engine.StaticMeshComponent|GetStaticMesh _asstatic_mesh_component))))
                (bind _asplaceable_base (Utilities|Casting|CastToPlaceableBase (Components|GetOwner _asstatic_mesh_component)))
                (if (not (Variables|/Script/ConanSandbox.BuildableBase|GetIsABrush _asplaceable_base))
                  (Utilities|Array|Add (LocalVariables|GetOverlappingBuildingStaticMeshes) (Variables|/Script/Engine.StaticMeshComponent|GetStaticMesh _asstatic_mesh_component)))))))
        (Variables|/Script/Engine.PrimitiveComponent|SetbGenerateOverlapEvents _overlapplaceablesboxchecker true)
        (Utilities|Array|AppendArray (LocalVariables|GetOverlappingActors) (Collision|GetOverlappingActors _overlapplaceablesboxchecker "/Game/Systems/Building/Placeables/BP_Master_Placeables.BP_Master_Placeables_C" :!class /Script/Engine.PrimitiveComponent))
        (if (Variables|Default|GetUseSecondaryPlaceablesBoxChecker)
          (Variables|/Script/Engine.PrimitiveComponent|SetbGenerateOverlapEvents _secondaryoverlapplaceablesboxchecker true)
          (Utilities|Array|AppendArray (LocalVariables|GetOverlappingActors) (Collision|GetOverlappingActors _secondaryoverlapplaceablesboxchecker "/Game/Systems/Building/Placeables/BP_Master_Placeables.BP_Master_Placeables_C" :!class /Script/Engine.PrimitiveComponent))
          (Variables|/Script/Engine.PrimitiveComponent|SetbGenerateOverlapEvents (Variables|Default|GetSecondaryOverlapPlaceablesBoxChecker) false))
        (Variables|/Script/Engine.PrimitiveComponent|SetbGenerateOverlapEvents (Variables|Default|GetOverlapPlaceablesBoxChecker) false)
        (for _array_element_3 (Variables|Default|GetCanUpgradeFrom)
          (bind _returnvalue_5 (Utilities|Array|RemoveItem _overlappingbuildingstaticmeshes _array_element_3))
          (if _returnvalue_5
            (LocalVariables|SetFoundUpgradeable true)))
        (if (and (== (Utilities|Array|Length _overlappingbuildingstaticmeshes) 0) (== (Utilities|Array|Length (LocalVariables|GetOverlappingActors)) 0))
          (if (Variables|Default|GetMustSnapToExistingBuilding)
            (if (Variables|Default|GetIsSnappedToSocket)
              _
              (else
                (return (Utilities|String|ToString(Text) (Variables|Default|GetError_Not_Snapped)) "Fail"))))
          (if (LocalVariables|GetFoundUpgradeable)
            (if (< _returnvalue_4 (Utilities|Enum|LiteralenumECanBePlacedResult "Fail"))
              (return "" "Success_Update")
              (else
                _)))
          (return _failedmessage _returnvalue_4)
          (else
            (return (Utilities|String|ToString(Text) (Variables|Default|GetError_Overlapping_Text)) "Fail_Overlaps")))))
    (else
      (return (Utilities|String|ToString(Text) (Variables|Default|GetError_BelowGround)) "Fail"))))