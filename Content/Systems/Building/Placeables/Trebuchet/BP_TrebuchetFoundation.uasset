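; Foundation actor for a buildable trebuchet in the placeables building system, tracking the parts that make up the siege engine.
; RegisterPart switches on part type to store the baseplate, arm, counterweight or sling in the trebuchet struct.
; It then prints a debug message naming the registered part and returns the foundation itself to the caller.
; BeginPlay, overlap, Tick and construction only call their parent versions.
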(event EventBeginPlay
  (|CallParentFunction))

(event Collision|EventActorBeginOverlap
  (params (OtherActor :type Actor%20Object%20Reference))
  (|CallParentFunction OtherActor))

(event EventTick
  (params (DeltaSeconds :type Float%20%28single-precision%29))
  (|CallParentFunction DeltaSeconds))

(fn ConstructionScript
  (|CallParentFunction))

(fn RegisterPart
  (params (PartType :type ETrebuchetParts%20Enum :default "NewEnumerator0") (Part :type Actor%20Object%20Reference))
  (LocalVariables|SetLPartType PartType)
  (LocalVariables|SetLPartToRegister Part)
  (Utilities|FlowControl|Sequence
    (:then_0
      (switch Utilities|FlowControl|Switch|SwitchonETrebuchetParts (LocalVariables|GetLPartType)
        (:NewEnumerator1
          (Utilities|Struct|SetmembersinTrebuchetStruct (Variables|Default|GetTrebuchetStruct) (LocalVariables|GetLPartToRegister)))
        (:NewEnumerator3
          (Utilities|Struct|SetmembersinTrebuchetStruct (Variables|Default|GetTrebuchetStruct) (LocalVariables|GetLPartToRegister)))
        (:NewEnumerator4
          (Utilities|Struct|SetmembersinTrebuchetStruct (Variables|Default|GetTrebuchetStruct) (LocalVariables|GetLPartToRegister)))
        (:NewEnumerator5
          (Utilities|Struct|SetmembersinTrebuchetStruct (Variables|Default|GetTrebuchetStruct) (LocalVariables|GetLPartToRegister)))))
    (:then_1
      (Development|PrintString (Utilities|String|Append (Utilities|GetDisplayName self) " Registered part: " (Utilities|GetDisplayName (LocalVariables|GetLPartToRegister))))
      (return self))))