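; Foundation building piece that decides whether it can be placed, extending the parent's CanBePlaced check.
; Downward box traces look for non-water landscape or static mesh actors, or instanced foundation, sealing or pillar meshes beneath it.
; Either support keeps the parent's result, otherwise placement fails; non-server instances skip the traces while loading.
; The resource-foliage blocking check is disconnected, so it never rejects placement.
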(event EventBeginPlay)

(event EventActorBeginOverlap
  (params (OtherActor :type Actor%20Object%20Reference)))

(event EventTick
  (params (DeltaSeconds :type Float%20%28single-precision%29)))

(fn ConstructionScript
  (|CallParentFunction))

(fn CanbePlaced
  (params (AttachTo :type Buildable%20Base%20Object%20Reference) (InstanceIndex :type Integer))
  (bind _checkforvalidbuildingsupport (Variables|Default|GetCheckForValidBuildingSupport))
  (bind _checkforlandscapeboxchecker (Variables|Default|GetCheckForLandscapeBoxChecker))
  (bind _returnvalue (Transformation|GetWorldLocation _checkforvalidbuildingsupport))
  (bind _returnvalue_2 (Transformation|GetWorldLocation _checkforlandscapeboxchecker))
  (bind (_x _y _z) (Math|Vector|BreakVector _returnvalue))
  (bind (_x_2 _y_2 _z_2) (Math|Vector|BreakVector _returnvalue))
  (bind (_x_3 _y_3 _z_3) (Math|Vector|BreakVector _returnvalue_2))
  (bind (_x_4 _y_4 _z_4) (Math|Vector|BreakVector _returnvalue_2))
  (bind (_failedmessage _returnvalue_3) (|CallParentFunction AttachTo InstanceIndex))
  (if (Networking|IsServer)
    (if (< (Math|Conversions|ToInteger(Byte) _returnvalue_3) (Math|Conversions|ToInteger(Byte) (Utilities|Enum|LiteralenumECanBePlacedResult "Fail")))
      _
      (else
        (return _failedmessage _returnvalue_3)))
    (elif (Variables|Default|Getm_IsLoading)
      (if (< (Math|Conversions|ToInteger(Byte) _returnvalue_3) (Math|Conversions|ToInteger(Byte) (Utilities|Enum|LiteralenumECanBePlacedResult "Fail")))
        (return "" "Success")
        (else
          (return _failedmessage _returnvalue_3)))
      (else
        _)))
  (Utilities|Array|Clear (Variables|Default|GetFoundLandscape))
  (Utilities|Array|Clear (Variables|Default|GetHitResourceActor))
  (Utilities|Array|Clear (Variables|Default|GetFoundFoundation))
  (bind _outhits (Class|KismetSystemLibrary|BoxTraceMulti (Math|Vector|MakeVector _x_4 _y_4 (+ _z_4 128.0)) (Math|Vector|MakeVector _x_3 _y_3 (- _z_3 32.0)) (Variables|/Script/Engine.BoxComponent|GetBoxExtent _checkforlandscapeboxchecker) (Transformation|GetWorldRotation _checkforlandscapeboxchecker) "TraceTypeQuery1" false 0 "None" true))
  (for _array_element _outhits
    (Utilities|Array|Add (Variables|Default|GetFoundLandscape) (and (Math|Boolean|ORBoolean (== (Utilities|GetClass (.HitActor (Collision|BreakHitResult _array_element))) "/Script/Landscape.Landscape") (== (Utilities|GetClass (.HitActor (Collision|BreakHitResult _array_element))) "/Script/Landscape.LandscapeProxy") (== (Utilities|GetClass (.HitActor (Collision|BreakHitResult _array_element))) "/Script/Engine.StaticMeshActor")) (not (Utilities|Array|ContainsItem (Variables|/Script/Engine.Actor|GetTags (.HitActor (Collision|BreakHitResult _array_element))) "Water")))))
  ;[1 0.04911 0] Build on top of foundations - remember to enable for triangles too
  (Utilities|Array|Clear (Variables|Default|GetFoundFoundation))
  (bind _outhits_2 (Class|KismetSystemLibrary|BoxTraceMulti (Math|Vector|MakeVector _x_2 _y_2 _z_2) (Math|Vector|MakeVector _x _y (- _z 32.0)) (Variables|/Script/Engine.BoxComponent|GetBoxExtent _checkforvalidbuildingsupport) (Transformation|GetWorldRotation _checkforvalidbuildingsupport) "TraceTypeQuery3" false 0 "None" true))
  (for _array_element_2 _outhits_2
    (bind _asinstanced_building_component (Utilities|Casting|CastToInstancedBuildingComponent (.HitComponent (Collision|BreakHitResult _array_element_2))))
    (Utilities|Array|Add (Variables|Default|GetFoundFoundation) (Utilities|Array|ContainsItem (Utilities|Array|MakeArray "/Game/Environment/Player_built/Meshes/SM_tier1_foundation.SM_tier1_foundation" "/Game/Environment/Player_built/Meshes/SM_tier2_foundation.SM_tier2_foundation" "/Game/Environment/Player_built/Meshes/SM_tier3_foundation.SM_tier3_foundation" "/Game/Environment/Player_built/Meshes/SM_tier1_sealing.SM_tier1_sealing" "/Game/Environment/Player_built/Meshes/SM_tier2_sealing.SM_tier2_sealing" "/Game/Environment/Player_built/Meshes/SM_tier3_sealing.SM_tier3_sealing" "/Game/Environment/Player_built/Meshes/SM_tier1_pillar.SM_tier1_pillar" "/Game/Environment/Player_built/Meshes/SM_tier2_pillar.SM_tier2_pillar" "/Game/Environment/Player_built/Meshes/SM_tier3_pillar.SM_tier3_pillar") (Variables|/Script/Engine.StaticMeshComponent|GetStaticMesh _asinstanced_building_component))))
  (if (and (or (Utilities|Array|ContainsItem (Variables|Default|GetFoundFoundation) true) (Utilities|Array|ContainsItem (Variables|Default|GetFoundLandscape) true)) (not (Utilities|Array|ContainsItem (Variables|Default|GetHitResourceActor) true)))
    (return _failedmessage _returnvalue_3)
    (else
      (return (Utilities|String|ToString(Text) (Variables|Default|GetError_CouldntFindLandscape)) "Fail"))))