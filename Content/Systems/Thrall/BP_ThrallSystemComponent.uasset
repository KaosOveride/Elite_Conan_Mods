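; Thrall system component that lets players preview, validate and place thralls from shortcut bar items.
; While placing, a non-replicated brush actor follows a camera trace each tick, and a failed check shows the blocked reason.
; The server spawns an AI NPC or plain actor, applies layout and ownership, then saves it or destroys it if invalid.
; Exclusion-radius checks use thrall home locations on the server and current locations on clients.
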(event Custom|Server%20Place%20Thrall
  (params (WorldPosition :type Transform) (ThrallItemInventory :type Item%20Inventory%20Object%20Reference) (ThrallItemIndex :type Integer))
  (bind (_location _rotation) (Math|Transform|BreakTransform WorldPosition))
  (bind _returnvalue (Class|ItemInventory|GetItem ThrallItemInventory ThrallItemIndex))
  ;[1 1 1] ServerPlaceThrall
  (Utilities|IsValid ThrallItemInventory
    (:Is%20Valid
      (Utilities|IsValid _returnvalue
        (:Is%20Valid
          (bind _asthrall_item (Utilities|Casting|CastToThrallItem _returnvalue)
            (:then
              (Variables|Default|SetSourceThrallItem _asthrall_item)
              (bind _valid (CallFunction|CheckValidPlacement (.Location (Math|Transform|BreakTransform WorldPosition)) true))
              (if _valid
                (Utilities|IsValid (Class|ThrallItem|GetThrallBehaviorTree (Variables|Default|GetSourceThrallItem))
                  (:Is%20Valid
                    ;[1 1 1] Spawning an NPC
                    (bind _aspawn (Utilities|Casting|CastToPawnClass (Class|ThrallItem|GetThrallActorClass (Variables|Default|GetSourceThrallItem))))
                    (bind _returnvalue_2 (AI|SpawnAIFromClass _aspawn "/Game/Systems/AI/AI_Controllers/AI_Controller_NPC.AI_Controller_NPC_C" (Class|ThrallItem|GetThrallBehaviorTree (Variables|Default|GetSourceThrallItem)) _location _rotation true))
                    (bind _output_get (Variables|Default|SetSpawnedActor _returnvalue_2))
                    (bind _asconan_character (Utilities|Casting|CastToConanCharacter _output_get)
                      (:then
                        (Class|ThrallItem|SetupThrallfromItem (Variables|Default|GetSourceThrallItem) _asconan_character)
                        (bind _returnvalue_3 (Class|ThrallItem|GetThrallTableRow (Variables|Default|GetSourceThrallItem)))
                        (bind _asbase_npc (Utilities|Casting|CastToBaseNPC (Variables|Default|GetSpawnedActor)))
                        (bind _asbp_npcbehavior_parameters (Utilities|Casting|CastToBP_NPCBehaviorParametersClass (.NPCBehaviorParameters (Utilities|Struct|BreakThrallTableRow _returnvalue_3))))
                        (bind _returnvalue_4 (Game|ConstructObjectfromClass _asbp_npcbehavior_parameters (Variables|Default|GetSpawnedActor)))
                        (CallFunction|ConfigureSpawnedNPC "NewEnumerator3" true _asbase_npc 0 0 0.0 (Transformation|GetActorLocation _asbase_npc) 0 0 _returnvalue_4 true)
                        (bind _returnvalue_5 (Class|UniqueID|GenerateUniqueID :!label _label))
                        (Class|DreamworldBlueprints|SetUniqueID (Variables|Default|GetSpawnedActor) _returnvalue_5)
                        (bind _returnvalue_6 (Class|ThrallSystemComponent|FindorSetupThrallComponent (Variables|Default|GetSpawnedActor) (Variables|Default|GetSourceThrallItem)))
                        (bind (_debugtext _displayfailtext _returnvalue_7) (CallFunction|CanbePlaced _returnvalue_6))
                        (if (Utilities|Enum|Equal(Enum) _returnvalue_7 "Success")
                          (bind _returnvalue_8 (Class|ThrallItem|GetThrallTableRow (Variables|Default|GetSourceThrallItem)))
                          (bind _asthrall_npcinterface (Utilities|Casting|CastToThrallNPCInterface (Variables|Default|GetSpawnedActor))
                            (:then
                              (Default|SetThrallComponentClass _asthrall_npcinterface (.ThrallComponent (Utilities|Struct|BreakThrallTableRow _returnvalue_8))))
                            (:CastFailed
                              _))
                          (bind _asbp_thrall_component (Utilities|Casting|CastToBP_ThrallComponent _returnvalue_6))
                          (bind _asi_has_character_layout_interface (Utilities|Casting|CastToI_HasCharacterLayoutInterface (Variables|Default|GetSpawnedActor))
                            (:then
                              (Default|SetCharacterLayout _asi_has_character_layout_interface (Variables|/Script/ConanSandbox.ThrallItem|GetThrallCharLayout (Variables|Default|GetSourceThrallItem))))
                            (:CastFailed
                              (bind _asbp_thrall_component_with_layout (Utilities|Casting|CastToBP_ThrallComponentWithLayout _asbp_thrall_component)
                                (:then
                                  (Variables|/Game/Systems/Thrall/BP_ThrallComponentWithLayout.BP_ThrallComponentWithLayout_C|SetThrallCharLayout _asbp_thrall_component_with_layout (Variables|/Script/ConanSandbox.ThrallItem|GetThrallCharLayout (Variables|Default|GetSourceThrallItem)))
                                  (Default|ApplyLayout _asbp_thrall_component_with_layout))
                                (:CastFailed
                                  _))))
                          (Variables|/Script/ConanSandbox.ThrallComponent|SetThrallInfo _asbp_thrall_component (Variables|/Script/ConanSandbox.ThrallItem|GetThrallInfo (Variables|Default|GetSourceThrallItem)))
                          (bind _asconan_character_2 (Utilities|Casting|CastToConanCharacter (Components|GetOwner)))
                          (bind _returnvalue_9 (Class|ConanCharacter|GetPrioritizedUID _asconan_character_2))
                          (Class|ThrallComponent|SetOwnerUniqueID _asbp_thrall_component _returnvalue_9)
                          (Class|ThrallComponent|ClaimLand _asbp_thrall_component)
                          (Class|ThrallSystemComponent|ConsumeThrallResource)
                          (Class|WorldPersistenceComponent|SaveActor (Variables|Default|GetSpawnedActor))
                          (else
                            (bind _asconan_character_3 (Utilities|Casting|CastToConanCharacter (Components|GetOwner))
                              (:then
                                (Class|ConanCharacter|ClientHUDShowFIFO _asconan_character_3 _displayfailtext))
                              (:CastFailed
                                _))
                            (Actor|DestroyActor (Variables|Default|GetSpawnedActor)))))
                      (:CastFailed
                        (Class|LoggerLibrary|DWLogString "ServerPlaceThrall: Tried to spawn an NPC that wasn't a ConanCharacter" "Thrall" "INFOL_DATAERROR"))))
                  (:Is%20Not%20Valid
                    ;[1 1 1] Spawning an Actor
                    (bind _returnvalue_10 (Game|SpawnActorfromClass (Class|ThrallItem|GetThrallActorClass (Variables|Default|GetSourceThrallItem)) WorldPosition "Undefined" 0 0))
                    (Variables|Default|SetSpawnedActor _returnvalue_10)
                    (goto _label)))
                (else
                  (bind _asconan_character_4 (Utilities|Casting|CastToConanCharacter (Components|GetOwner)))
                  (Class|ConanCharacter|ClientHUDShowFIFO _asconan_character_4 (Utilities|Text|MakeLiteralText "There's a thrall placed too close by")))))
            (:CastFailed
              (Class|LoggerLibrary|DWLogString "ServerPlaceThrall: Source item is not a thrall item" "Thrall" "INFOL_CODEWARNING"))))
        (:Is%20Not%20Valid
          (Class|LoggerLibrary|DWLogString "ServerPlaceThrall: Could not find chosen thrall item" "Thrall" "INFOL_CODEWARNING"))))
    (:Is%20Not%20Valid
      (Class|LoggerLibrary|DWLogString "ServerPlaceThrall: Trying to spawn thrall from invalid inventory" "Thrall" "INFOL_CODEWARNING"))))

(event EventBeginPlay)

(event EventTick
  (params (DeltaSeconds :type Float%20%28single-precision%29))
  (bind _returnvalue (Class|GUIModuleController|GetGUIModuleController))
  (bind _returnvalue_2 (Components|GetOwner))
  (bind _brushactor (Variables|Default|GetBrushActor))
  (bind _returnvalue_3 (Actor|GetComponentsByClass _returnvalue_2 "/Script/ConanSandbox.AdjustableCameraComponent"))
  (bind _item (Utilities|Array|Get(acopy) _returnvalue_3))
  (bind _returnvalue_4 (Transformation|GetWorldLocation _item))
  ;[1 1 1] EventTick
  (if (Variables|Default|GetIsPlacingThrall)
    (if (> (Utilities|Array|Length _returnvalue_3) 0)
      (bind _outhit (Class|KismetSystemLibrary|SphereTraceSingleNEW _returnvalue_4 (+ _returnvalue_4 (* (Math|Vector|GetForwardVector _item) (Variables|Default|GetPlaceableRange))) 0.0 "TraceTypeQuery1" false (Utilities|Array|MakeArray (Variables|Default|GetBrushActor)) "None" true))
      (bind _output_get (Variables|Default|SetBrushTransform (Math|Transform|MakeTransform (+ (.Location (Collision|BreakHitResult _outhit)) (Math|Vector|MakeVector 0.0 0.0 (Variables|Default|GetBrushGroundOffset))) (Math|Rotator|CombineRotators (Transformation|GetActorRotation _returnvalue_2) (Variables|Default|GetRotation)) "1,1,1.000000")))
      (Transformation|SetActorTransform _brushactor _output_get)
      (bind (_debugtext _displayfailtext _returnvalue_5) (CallFunction|CanbePlaced (Utilities|Array|Get(acopy) (Actor|GetComponentsByClass _brushactor "/Script/ConanSandbox.ThrallComponent"))))
      (if (Utilities|Enum|Equal(Enum) _returnvalue_5 "Success")
        (Class|GUIModuleController|ActivateModule _returnvalue "CanBuildIndicator" false)
        (else
          (bind _returnvalue_6 (Class|GUIModuleController|ActivateModule _returnvalue "CanBuildIndicator" true))
          (bind _asw_can_build_indicator (Utilities|Casting|CastToW_CanBuildIndicator _returnvalue_6))
          (Default|SetBlockedReason _asw_can_build_indicator _displayfailtext))))))

(fn ShowThrallPlaceable
  (params (item :type Thrall%20Item%20Object%20Reference))
  (bind _returnvalue (|CallParentFunction item))
  (bind _output_get (Variables|Default|SetBrushActor _returnvalue))
  (Networking|SetReplicates _output_get false)
  (if (> (Utilities|Array|Length (Actor|GetComponentsByClass _returnvalue "/Game/Systems/Thrall/BP_ThrallComponentWithLayout.BP_ThrallComponentWithLayout_C")) 0)
    (Variables|/Game/Systems/Thrall/BP_ThrallComponentWithLayout.BP_ThrallComponentWithLayout_C|SetThrallCharLayout (Utilities|Array|Get(acopy) (Actor|GetComponentsByClass _returnvalue "/Game/Systems/Thrall/BP_ThrallComponentWithLayout.BP_ThrallComponentWithLayout_C")) (Variables|/Script/ConanSandbox.ThrallItem|GetThrallCharLayout item))
    (Default|ApplyLayout (Utilities|Array|Get(acopy) (Actor|GetComponentsByClass _returnvalue "/Game/Systems/Thrall/BP_ThrallComponentWithLayout.BP_ThrallComponentWithLayout_C")))
    (else
      (bind _asi_has_character_layout_interface (Utilities|Casting|CastToI_HasCharacterLayoutInterface (Variables|Default|GetBrushActor))
        (:then
          (Default|SetCharacterLayout _asi_has_character_layout_interface (Variables|/Script/ConanSandbox.ThrallItem|GetThrallCharLayout item)))
        (:CastFailed
          _))))
  (bind _ascapsule_collision (Utilities|Casting|CastToCapsuleComponent (VehicleSound|GetRootComponent (Variables|Default|GetBrushActor)))
    (:then
      (Variables|Default|SetBrushGroundOffset (Components|Capsule|GetScaledCapsuleHalfHeight _ascapsule_collision)))
    (:CastFailed
      (Variables|Default|SetBrushGroundOffset 0.0)))
  (bind _asbase_bpchar_interface (Utilities|Casting|CastToBaseBPCharInterface (Variables|Default|GetBrushActor))
    (:then
      (bind _isnpc (Default|CheckIsNPC _asbase_bpchar_interface))
      (if _isnpc
        (return (Variables|Default|GetBrushActor))
        (else
          _)))
    (:CastFailed
      _))
  (Collision|SetCollisionEnabled (Utilities|Array|Get(acopy) (Actor|GetComponentsbyTag (Variables|Default|GetBrushActor) "/Script/Engine.SkeletalMeshComponent" "MainMesh")) "NoCollision")
  (Components|Animation|PlayAnimation (Utilities|Array|Get(acopy) (Actor|GetComponentsbyTag (Variables|Default|GetBrushActor) "/Script/Engine.SkeletalMeshComponent" "MainMesh")) "/Game/Characters/humans/animations/movement/male/normal/A_normal_idle_3rd_M.A_normal_idle_3rd_M" true)
  (return (Variables|Default|GetBrushActor)))

(fn HideThrallPlaceable
  (Actor|DestroyActor (Variables|Default|GetBrushActor))
  (bind _returnvalue (|CallParentFunction))
  (Class|GUIModuleController|ActivateModule (Class|GUIModuleController|GetGUIModuleController) "CanBuildIndicator" false)
  (return _returnvalue))

(fn RotateThrall
  (params (Rotation :type Float%20%28single-precision%29))
  (Variables|Default|SetRotation (Math|Rotator|MakeRotator (.Roll (Math|Rotator|BreakRotator (Variables|Default|GetRotation))) (.Pitch (Math|Rotator|BreakRotator (Variables|Default|GetRotation))) (+ (* Rotation 5.0) (.Yaw (Math|Rotator|BreakRotator (Variables|Default|GetRotation)))))))

(fn PlaceThrall
  (bind _returnvalue (Components|GetOwner))
  (bind _returnvalue_2 (Actor|GetComponentsbyTag _returnvalue "/Script/ConanSandbox.ItemInventory" "ShortcutBar"))
  (bind _item (Utilities|Array|Get(acopy) _returnvalue_2))
  (bind _returnvalue_3 (CallFunction|CanbePlaced (Utilities|Array|Get(acopy) (Actor|GetComponentsByClass (Variables|Default|GetBrushActor) "/Script/ConanSandbox.ThrallComponent"))))
  (if (Utilities|Enum|Equal(Enum) _returnvalue_3 "Success")
    (Actor|DestroyActor (Variables|Default|GetBrushActor))
    (if (> (Utilities|Array|Length _returnvalue_2) 0)
      (CallFunction|ServerPlaceThrall (Variables|Default|GetBrushTransform) _item (Class|ItemInventory|GetItemIndex _item (Variables|Default|GetCurrentThrallItem)))
      (else
        (Class|LoggerLibrary|DWLogString "PlaceThrall: Can't find ShorcutBar" "Thrall" "INFOL_DATAERROR")))
    (Variables|Default|SetIsPlacingThrall false)
    (Variables|Default|SetBrushActor 0)
    (bind _returnvalue_4 (|CallParentFunction))
    (return _returnvalue_4)
    (else
      (return false))))

(fn CheckValidPlacement
  (params (Location :type Vector) (IsServer :type Boolean) (PlacingActor :type Actor%20Object%20Reference))
  (LocalVariables|SetlocalLocation Location)
  (if IsServer
    (bind _actorsinrange (Class|AILODSystem|AppendAILODActorsinRange Location (Variables|/Game/Systems/BP_ServerSettings.BP_ServerSettings_C|GetThrallExclusionRadius (|GetServerSettings))))
    (for _array_element _actorsinrange
      ;[1 1 1] Only check actual thrall npcs
      (if (> (Utilities|Array|Length (Actor|GetComponentsByClass _array_element "/Script/ConanSandbox.ThrallComponent")) 0)
        (if (!= _array_element PlacingActor)
          (Utilities|Array|Add (LocalVariables|GetThrallActors) _array_element))))
    (for _array_element_2 (LocalVariables|GetThrallActors)
      (bind _aspawn (Utilities|Casting|CastToPawn _array_element_2))
      (bind _asconan_aicontroller (Utilities|Casting|CastToConanAIController (Pawn|GetController _aspawn)))
      ;[1 1 1] Found a thrall too close by, return false
      (if (<= (Math|Vector|VectorLengthSquared (- (AI|Components|Blackboard|GetValueasVector (AI|GetBlackboard _asconan_aicontroller) (Class|ConanAIController|GetBBKeyName _asconan_aicontroller "HomeLocation")) (LocalVariables|GetlocalLocation))) (Math|Float|Square (Variables|/Game/Systems/BP_ServerSettings.BP_ServerSettings_C|GetThrallExclusionRadius (|GetServerSettings))))
        (return false)))
    (return true)
    (else
      ;[1 1 1] On the client let's just check every NPC we have, current location of the NPC. We don't have their home location here.
      (bind _outactors (Actor|GetAllActorswithInterface "/Game/Systems/Thrall/ThrallNPCInterface.ThrallNPCInterface_C"))
      (for _array_element_3 _outactors
        (if (!= _array_element_3 (Variables|Default|GetBrushActor))
          (if (<= (Math|Vector|VectorLengthSquared (- (Transformation|GetActorLocation _array_element_3) (LocalVariables|GetlocalLocation))) (Math|Float|Square (Variables|/Game/Systems/BP_ServerSettings.BP_ServerSettings_C|GetThrallExclusionRadius (|GetServerSettings))))
            (return false))))
      (return true))))

(fn CanbePlaced
  (params (ThrallComponent :type Thrall%20Component%20Object%20Reference))
  (bind _returnvalue (Components|GetOwner ThrallComponent))
  (bind (_debugtext _displayfailtext _returnvalue_2) (|CallParentFunction ThrallComponent))
  (if (Utilities|Enum|NotEqual(Enum) _returnvalue_2 "Success")
    (return _debugtext _displayfailtext _returnvalue_2)
    (else
      (bind _valid (CallFunction|CheckValidPlacement (Transformation|GetActorLocation _returnvalue) (Networking|IsServer) _returnvalue))
      (if _valid
        (return "" "" "Success")
        (else
          (return "Failed due to existing thralls being within the exclusion zone" "Too close to another Thrall" "Fail"))))))