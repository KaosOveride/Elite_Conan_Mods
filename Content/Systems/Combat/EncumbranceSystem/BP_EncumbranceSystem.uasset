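; Character encumbrance component that tracks carried item weight, sets a stamina effect per tier and immobilizes overloaded characters.
; On data load it totals backpack, equipment and hotbar items, then applies server-side deltas from inventory add, remove and stack-change signals, skipping shortcuts.
; The load ratio against base plus progression bonus picks the tier.
; The top tier disables movement with a throttled HUD warning; recovery uses Falling mode to dodge a replication bug.
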(event EventDataLoaded
  (|CallParentFunction)
  (|SetCharacterMovement
    (:exit
      (|SetProgressionSystem
        (:else
          (|SetBackpackInventory)
          (|SetEquipmentInventory)
          (|SetHotbarInventory)
          (|ProcessInventories
            (:Completed
              (|BindInventorySignals))))))))

(fn HandleCharacterEncumbrance
  (if (Networking|IsServer)
    (LocalVariables|SetCurrentEncumbranceLevel (/ (Variables|Default|GetEncumbranceCurrent) (CallFunction|GetEncumbranceMax)))
    (Variables|Default|SetCurrentEncumbranceTier "Tier4")
    (bind (_array_element _array_index) (Utilities|Array|ForEachLoopwithBreak (Variables|Default|GetEncumbranceTierThresholds) :!label _label)
      (:LoopBody
        (if (>= _array_element (LocalVariables|GetCurrentEncumbranceLevel))
          (Variables|Default|SetCurrentEncumbranceTier (Utilities|Enum|ByteToEnumEEncumbranceTiers (Math|Conversions|ToByte(Integer) _array_index)))
          (goto _label Break)))
      (:Completed
        (CallFunction|HandleOverWeight)))))

(fn GetEncumbranceStaminaEffect
  ;[1 1 1] Check for cheats like a c++ maestro =3
  (bind _asconan_character (Utilities|Casting|CastToConanCharacter (Components|GetOwner))
    (:then
      (if (Variables|/Script/ConanSandbox.ConanCharacter|GetSprintNoCost _asconan_character)
        (return 0.0)
        (else
          _)))
    (:CastFailed
      _))
  (return (Utilities|Array|Get(acopy) (Variables|Default|GetEncumbranceStaminaEffect) (Math|Conversions|ToInteger(Byte) (Variables|Default|GetCurrentEncumbranceTier)))))

(fn HandleOverWeight
  (bind _comp (CallFunction|GetCharacterMovementComp))
  (if (Utilities|Enum|Equal(Enum) (Variables|Default|GetCurrentEncumbranceTier) "Tier4")
    (Pawn|Components|CharacterMovement|DisableMovement (CallFunction|GetCharacterMovementComp))
    (bind _asconan_character (Utilities|Casting|CastToConanCharacter (Components|GetOwner)))
    (if (< (+ (Variables|Default|GetTimeFIDOSinceLast) (Variables|Default|GetTimeFIFOCooldown)) (Utilities|Time|GetGameTimeinSeconds))
      (Class|ConanCharacter|ClientHUDShowFIFO _asconan_character (Utilities|Text|FormatText "You are carrying too much and cannot move"))
      (Variables|Default|SetTimeFIDOSinceLast (Utilities|Time|GetGameTimeinSeconds)))
    (elif (Utilities|Enum|Equal(Enum) (Variables|/Script/Engine.CharacterMovementComponent|GetMovementMode _comp) "MOVE_None")
      ;[1 1 1] Set to falling rather than walking to workaround a replication bug in unreal
      (Pawn|Components|CharacterMovement|SetMovementMode _comp "MOVE_Falling" 0))))

(fn HandleItemEncumbrance
  (params (GameItem :type Game%20Item%20Object%20Reference) (NewItem :type Boolean) (StackChangeDelta :type Integer))
  (Utilities|IsValid GameItem
    (:Is%20Valid
      (if (Networking|IsServer)
        (Utilities|FlowControl|Sequence
          (:then_0
            (LocalVariables|Setlocal%20GameItem GameItem))
          (:then_1
            (LocalVariables|Setlocal%20NewItem NewItem))
          (:then_2
            (LocalVariables|Setlocal%20StackChangeDelta StackChangeDelta))
          (:then_3
            (if (not (Class|GameItem|IsShortcut (LocalVariables|Getlocal%20GameItem)))
              (if (!= (LocalVariables|Getlocal%20StackChangeDelta) 0)
                ;[1 1 1] Handle Stack size change
                (LocalVariables|Setlocal%20WeightDelta (* (LocalVariables|Getlocal%20StackChangeDelta) (Class|GameItem|GetFloatStat (LocalVariables|Getlocal%20GameItem) "EncumbranceWeight")))
                (else
                  ;[1 1 1] Handle adding or removing whole items, including item with a stack
                  (LocalVariables|Setlocal%20WeightDelta (* (* (Math|Integer|SelectInt (Class|GameItem|GetIntStat (LocalVariables|Getlocal%20GameItem) "StackSize") 1 (> (Class|GameItem|GetIntStat (LocalVariables|Getlocal%20GameItem) "MaxStackSize") 0)) (Class|GameItem|GetFloatStat (LocalVariables|Getlocal%20GameItem) "EncumbranceWeight")) (Math|Float|SelectFloat 1.0 -1.0 (LocalVariables|Getlocal%20NewItem))))))
              (Variables|Default|SetEncumbranceCurrent (+ (Variables|Default|GetEncumbranceCurrent) (LocalVariables|Getlocal%20WeightDelta)))
              (CallFunction|HandleCharacterEncumbrance))))))))

(fn GetEncumbranceMax
  (bind _encumbrancebase (Variables|Default|GetEncumbranceBase))
  (bind _progressionsystem (Variables|Default|GetProgressionSystem))
  (Utilities|IsValid _progressionsystem
    (:Is%20Valid
      (return (+ _encumbrancebase (Variables|/Game/Systems/Progression/BP_ProgressionSystem.BP_ProgressionSystem_C|GetBonusEncumbrance _progressionsystem))))
    (:Is%20Not%20Valid
      (return _encumbrancebase))))

(fn OnRepEncumbranceCurrent
  (Default|CallSignalEncumbranceChanged))

(fn OnRepEncumbranceBase
  (Default|CallSignalEncumbranceChanged))

(fn GetCharacterMovementComp
  (bind _returnvalue (Components|GetOwner))
  (bind _returnvalue_2 (Actor|GetComponentsByClass _returnvalue "/Script/Engine.CharacterMovementComponent"))
  (bind _charactermovement (Variables|Default|GetCharacterMovement)
    (:then
      (return _charactermovement))
    (:else
      (if (> (Utilities|Array|Length _returnvalue_2) 0)
        (bind _output_get (Variables|Default|SetCharacterMovement (Utilities|Array|Get(acopy) _returnvalue_2)))
        (return _output_get)
        (else
          (return 0))))))

(event Custom|SignalItemIntStatChanged_Encumbrance
  (params (item :type Game%20Item%20Object%20Reference) (statID :type EItemIntStatID%20Enum) (statValue :type Integer) (deltaValue :type Integer))
  ;[1 1 1] Bind all inventories to Add Item and remove Item signals
  (if (Utilities|Enum|Equal(Enum) statID "StackSize")
    (CallFunction|HandleItemEncumbrance item false deltaValue)))

(event Custom|SignalItemAdded_Encumbrance
  (params (index :type Integer) (item :type Game%20Item%20Object%20Reference) (srcInventory :type Item%20Inventory%20Object%20Reference) (srcIndex :type Integer))
  ;[1 1 1] Bind all inventories to Add Item and remove Item signals
  (CallFunction|HandleItemEncumbrance item true))

(event Custom|SignalItemRemoved_Encumbrance
  (params (index :type Integer) (item :type Game%20Item%20Object%20Reference) (dstInventory :type Item%20Inventory%20Object%20Reference) (dstIndex :type Integer))
  ;[1 1 1] Bind all inventories to Add Item and remove Item signals
  (CallFunction|HandleItemEncumbrance item false))