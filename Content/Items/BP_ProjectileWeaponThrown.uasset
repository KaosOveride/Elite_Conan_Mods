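; BP_ProjectileWeaponThrown is a thrown projectile weapon item that manages its visibility and stack state when thrown.
; WeaponThrown hides the visual actor, zeroes the replicated stack size and, for items with a max stack of one, disables the item and flags it for deletion.
; WeaponAttackEnd runs once per throw, calling the parent and setting flagged items' stack size to -1, apparently to mark them for removal.
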(fn WeaponAttackEnd
  (if (not (Variables|Weapons|GetHasFinishedWeaponAttack))
    (bind _success (|CallParentFunction))
    (LocalVariables|Setlocal%20Success _success)
    (if (Variables|Weapons|GetDeleteAfterThrow)
      (Class|GameItem|SetIntStat "StackSize" -1 true)
      (LocalVariables|Setlocal%20Success true))
    (Variables|Weapons|SetHasFinishedWeaponAttack true)
    (return (LocalVariables|Getlocal%20Success))
    (else
      (return false))))

(fn WeaponThrown
  (Variables|Weapons|SetHasFinishedWeaponAttack false)
  (Rendering|SetActorHiddenInGame (Variables|Default|GetVisualActor) true)
  (Class|GameItem|SetIntStat "StackSize" 0 true)
  (if (not (== (Class|GameItem|GetIntStat "MaxStackSize") 1))
    _
    (else
      (Class|GameItem|Enable false)
      (Variables|Weapons|SetDeleteAfterThrow true)))
  (return true))